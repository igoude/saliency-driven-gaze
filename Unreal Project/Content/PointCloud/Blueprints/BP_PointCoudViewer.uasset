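; Point cloud viewer actor that renders a texture-encoded cloud with a saliency overlay and can play back timed texture sequences.
; Construction adds one mesh instance per texel, storing its index in custom data for the dynamic material.
; Tick pushes display parameters, keeps the actor ahead of the camera, and async-loads time-indexed saliency textures, plus scan textures for dynamic scenes.
; Playback ends on black saliency; the blocking UpdateTextures path is disconnected.
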(event `self.ReceiveBeginPlay`
  (bind _returnvalue (`KismetMaterialLibrary.CreateDynamicMaterialInstance` "/Game/PointCloud/Materials/M_PointCloudMaterial.M_PointCloudMaterial"))
  (bind _output_get (set `self.PointCloudMaterial` _returnvalue))
  (`MaterialInstanceDynamic.SetTextureParameterValue` _output_get "PointCoudTexture" (`self.PointCloudTexture`))
  (`MaterialInstanceDynamic.SetTextureParameterValue` _output_get "PointCoudSaliency" (`self.PointCloudSaliency`))
  (`PrimitiveComponent.SetMaterial` (`self.InstancedStaticMesh`) 0 _output_get))

(event `self.ReceiveTick`
  (params (DeltaSeconds :type "Float (single-precision)"))
  (bind _returnvalue (`GameplayStatics.GetPlayerCameraManager` 0))
  (bind _levelname (`self.LevelName`))
  (bind _texid (`self.TexID`))
  (bind _pointcloudmaterial (`self.PointCloudMaterial`))
  (bind _idstring_0 (`self.IDString_0`))
  (bind _idstring_0_2 (`self.IDString_0`))
  (bind _levelname_2 (`self.LevelName`))
  (bind _returnvalue_2 (`KismetStringLibrary.Conv_IntToString` _texid))
  (bind _returnvalue_3 (`KismetStringLibrary.Concat_StrStr` (`self.Name String`) "_scan"))
  (bind _returnvalue_4 (* (/ (`KismetMathLibrary.FFloor` (* (+ (`GameplayStatics.GetTimeSeconds`) 7.0) 1000.0)) 20) 20))
  (`|ExecutionSequence`
    (:`then_1`
      (`MaterialInstanceDynamic.SetScalarParameterValue` _pointcloudmaterial "SaliencyScale" (`self.SaliencyScale`))
      (`MaterialInstanceDynamic.SetScalarParameterValue` _pointcloudmaterial "Opacity" (`self.Opacity`))
      (`MaterialInstanceDynamic.SetScalarParameterValue` _pointcloudmaterial "CloudScale" (`self.Cloud Scaling`))
      (`MaterialInstanceDynamic.SetScalarParameterValue` _pointcloudmaterial "SplatSize" (`self.Splat Size`)))
    (:`then_2`
      (`self.K2_SetActorLocation` (+ (`self.K2_GetActorLocation` _returnvalue) (* (`self.GetActorForwardVector` _returnvalue) 50.0))))
    (:`then_3`
      (if (`self.StartPlayingSaliency`)
        (if (>= _returnvalue_4 (`self.TexID`))
          (set `self.TexID` _returnvalue_4)
          (`|ExecutionSequence`
            (:`then_0`
              (if (< _texid 10000)
                (set `self.IDString_0` (`KismetStringLibrary.Concat_StrStr` "0" _returnvalue_2))
                (else
                  (set `self.IDString_0` _returnvalue_2))))
            (:`then_1`
              (bind _object (`|LoadAsset` (`KismetSystemLibrary.Conv_SoftObjPathToSoftObjRef` (`KismetSystemLibrary.MakeSoftObjectPath` (`KismetStringLibrary.Concat_StrStr` "Texture2D'/Game/Textures/" _levelname "/" _levelname "-" _idstring_0 "." _levelname "-" _idstring_0 "'"))))
                (:`Completed`
                  (bind _astexture_2d (cast `Texture2D` _object))
                  (`MaterialInstanceDynamic.SetTextureParameterValue` (`self.PointCloudMaterial`) "PointCoudSaliency" _astexture_2d))))
            (:`then_2`
              (if (`self.DynamicScene`)
                (if false
                  (set `self.Name String` (`KismetStringLibrary.Split` _levelname_2 "_event"))
                  (else
                    (set `self.Name String` _levelname_2)))
                (bind _object_2 (`|LoadAsset` (`KismetSystemLibrary.Conv_SoftObjPathToSoftObjRef` (`KismetSystemLibrary.MakeSoftObjectPath` (`KismetStringLibrary.Concat_StrStr` "Texture2D'/Game/Textures/" _returnvalue_3 "/" _returnvalue_3 "-" _idstring_0_2 "." _returnvalue_3 "-" _idstring_0_2 "'"))))
                  (:`Completed`
                    (bind _astexture_2d_2 (cast `Texture2D` _object_2))
                    (`MaterialInstanceDynamic.SetTextureParameterValue` (`self.PointCloudMaterial`) "PointCoudTexture" _astexture_2d_2)))))
            (:`then_3`
              (if (>= (`self.TexID`) 35000)
                (set `self.StartPlayingSaliency` false)
                (`MaterialInstanceDynamic.SetTextureParameterValue` (`self.PointCloudMaterial`) "PointCoudSaliency" "/Game/MH/Common/Materials/T_Black_Linear.T_Black_Linear")))))))))

(fn `UpdateTextures`
  (locals (StartID :type Integer :default 7000) (EndID :type Integer :default 35000) (IDString :type String) (NameString :type String))
  (bind _levelname (`self.LevelName`))
  (bind _texid (`self.TexID`))
  (bind _levelname_2 (`self.LevelName`))
  (bind _idstring (`local.IDString`))
  (bind _idstring_2 (`local.IDString`))
  (bind _returnvalue (`KismetStringLibrary.Conv_IntToString` _texid))
  (bind (_lefts _rights _returnvalue_2) (`KismetStringLibrary.Split` _levelname_2 "_event"))
  (bind _returnvalue_3 (`KismetStringLibrary.Concat_StrStr` (`local.NameString`) "_scan"))
  (`|ExecutionSequence`
    (:`then_0`
      (if (< _texid 10000)
        (set `local.IDString` (`KismetStringLibrary.Concat_StrStr` "0" _returnvalue))
        (else
          (set `local.IDString` _returnvalue))))
    (:`then_1`
      (bind _returnvalue_4 (`KismetSystemLibrary.LoadAsset_Blocking` (`KismetSystemLibrary.Conv_SoftObjPathToSoftObjRef` (`KismetSystemLibrary.MakeSoftObjectPath` (`KismetStringLibrary.Concat_StrStr` "Texture2D'/Game/Textures/" _levelname "/" _levelname "-" _idstring "." _levelname "-" _idstring "'")))))
      (bind _astexture_2d (cast `Texture2D` _returnvalue_4))
      (`MaterialInstanceDynamic.SetTextureParameterValue` (`self.PointCloudMaterial`) "PointCoudSaliency" _astexture_2d))
    (:`then_2`
      (if (`self.DynamicScene`)
        (if _returnvalue_2
          (set `local.NameString` _lefts)
          (else
            (set `local.NameString` _levelname_2)))
        (bind _returnvalue_5 (`KismetSystemLibrary.LoadAsset_Blocking` (`KismetSystemLibrary.Conv_SoftObjPathToSoftObjRef` (`KismetSystemLibrary.MakeSoftObjectPath` (`KismetStringLibrary.Concat_StrStr` "Texture2D'/Game/Textures/" _returnvalue_3 "/" _returnvalue_3 "-" _idstring_2 "." _returnvalue_3 "-" _idstring_2 "'")))))
        (bind _astexture_2d_2 (cast `Texture2D` _returnvalue_5))
        (`MaterialInstanceDynamic.SetTextureParameterValue` (`self.PointCloudMaterial`) "PointCoudTexture" _astexture_2d_2)))
    (:`then_3`
      (if (>= (`self.TexID`) (`local.EndID`))
        (set `self.StartPlayingSaliency` false)
        (`MaterialInstanceDynamic.SetTextureParameterValue` (`self.PointCloudMaterial`) "PointCoudSaliency" "/Game/MH/Common/Materials/T_Black_Linear.T_Black_Linear")))))

(fn `UserConstructionScript`
  (bind _pointcloudtexture (`self.PointCloudTexture`))
  (bind _instancedstaticmesh (`self.InstancedStaticMesh`))
  (if (`KismetSystemLibrary.IsValid` _pointcloudtexture)
    (bind _output_get (set `self.NbPoints` (* (`Texture2D.Blueprint_GetSizeX` _pointcloudtexture) (`Texture2D.Blueprint_GetSizeY` _pointcloudtexture))))
    (while (< (`self.CurrentNbPoints`) _output_get)
      (`|ExecutionSequence`
        (:`then_0`
          (bind _returnvalue (`InstancedStaticMeshComponent.AddInstance` _instancedstaticmesh (`KismetMathLibrary.MakeTransform` (0.0 0.0 0.0) (struct) (`KismetMathLibrary.Conv_DoubleToVector` (`self.Splat Size`))) false))
          (`InstancedStaticMeshComponent.SetCustomDataValue` _instancedstaticmesh _returnvalue 0 (`KismetMathLibrary.Conv_IntToDouble` _returnvalue) false))
        (:`then_1`
          (`/Engine/EditorBlueprintResources/StandardMacros.IncrementInt` (`self.CurrentNbPoints`)))))))