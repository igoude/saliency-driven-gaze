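; Level point cloud generator that scans the surroundings with spherical line traces and exports hit positions as EXR textures.
; ScanAllScene traces in batches each tick, writing each impact XYZ as a render target pixel's RGB.
; Dynamic mode nearly freezes time dilation to capture numbered frames at fixed game-time intervals, quitting after the last.
; After the first dynamic export, only angles inside UpdateBox regions are re-traced.
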(event `self.ReceiveBeginPlay`
  (bind _theta_samples (`self.theta_samples`))
  (bind _phi_samples (`self.phi_samples`))
  (set `self.nb_points` (* _theta_samples _phi_samples))
  (bind _returnvalue (`KismetRenderingLibrary.CreateRenderTarget2D` _theta_samples _phi_samples))
  (set `self.Point Cloud Texture` _returnvalue)
  (set `self.phi_step` (/ 180.0 (`KismetMathLibrary.Conv_IntToDouble` (`self.phi_samples`))))
  (set `self.theta_step` (/ 360.0 (`KismetMathLibrary.Conv_IntToDouble` (`self.theta_samples`)))))

(event `self.ReceiveTick`
  (params (DeltaSeconds :type "Float (single-precision)"))
  (bind _returnvalue (`GameplayStatics.GetTimeSeconds`))
  (bind _id_iterator (`self.id_iterator`))
  (bind _id_iterator_2 (`self.id_iterator`))
  (bind _returnvalue_2 (`KismetStringLibrary.Conv_IntToString` _id_iterator_2))
  (bind _returnvalue_3 (* (/ (`KismetMathLibrary.FFloor` (* _returnvalue 1000.0)) 20) 20))
  (if (`self.Scan`)
    (if (`self.IsDynamic`)
      (if (`self.ReadyForNextFrame`)
        (if (and (>= _returnvalue 7.0) (>= _returnvalue_3 _id_iterator))
          (`GameplayStatics.SetGlobalTimeDilation` 0.0001)
          (set `self.ReadyForNextFrame` false)
          (`KismetSystemLibrary.PrintString` (`KismetStringLibrary.Concat_StrStr` (`KismetStringLibrary.Conv_DoubleToString` _returnvalue) " / " (`KismetStringLibrary.Conv_IntToString` _returnvalue_3) " / " (`KismetStringLibrary.Conv_IntToString` _id_iterator))))
        (else
          (`self.ScanAllScene`)
          (if (>= (`self.current_point_index`) (`self.nb_points`))
            (if (< _id_iterator_2 10000)
              (bind _returnvalue_4 (`GameplayStatics.GetCurrentLevelName` true))
              (`self.SaveTextureEvent` (`KismetStringLibrary.Concat_StrStr` _returnvalue_4 "/" _returnvalue_4 "-" (`KismetStringLibrary.Concat_StrStr` "0" _returnvalue_2)))
              (else
                (bind _returnvalue_5 (`GameplayStatics.GetCurrentLevelName` true))
                (`self.SaveTextureEvent` (`KismetStringLibrary.Concat_StrStr` _returnvalue_5 "/" _returnvalue_5 "-" _returnvalue_2))))
            (set `self.id_iterator` (+ (`self.id_iterator`) 20))
            (set `self.current_point_index` 0)
            (set `self.phi` -90.0)
            (set `self.theta` -90.0))))
      (else
        (`self.ScanAllScene`)
        (if (>= (`self.current_point_index`) (`self.nb_points`))
          (bind _returnvalue_6 (`GameplayStatics.GetCurrentLevelName` true))
          (`self.SaveTextureEvent` _returnvalue_6))))))

(event `SaveTextureEvent`
  (params (FileName :type String))
  (if (`self.Scan`)
    (`ImageWriteBlueprintLibrary.ExportToDisk` (`self.Point Cloud Texture`) (`KismetStringLibrary.Concat_StrStr` (`KismetSystemLibrary.GetProjectDirectory`) "/Content/Textures/" FileName ".exr") (make `ImageWriteOptions` "EXR" (delegate `ExportToDiskCompleteEvent`) 1))))

(event `ExportToDiskCompleteEvent`
  (params (bSuccess :type Boolean))
  (if bSuccess
    (set `self.ReadyForNextFrame` true)
    (`GameplayStatics.SetGlobalTimeDilation` 0.05)
    (set `self.IsFirstScan` false)
    (if (>= (`self.id_iterator`) 35000)
      (`KismetSystemLibrary.QuitGame` null "Quit"))))

(fn `ScanAllScene`
  (locals (iterator_l :type Integer) (should_update_l :type Boolean))
  (bind _returnvalue (`self.K2_GetActorLocation`))
  (bind _current_point_index (`self.current_point_index`))
  (bind _theta_samples (`self.theta_samples`))
  (bind _updatebox (`self.UpdateBox`))
  (bind _returnvalue_2 (+ (`self.theta`) 90.0))
  (bind _returnvalue_3 (+ (`self.phi`) 90.0))
  (bind _returnvalue_4 (`KismetMathLibrary.MakeVector2D` (`KismetMathLibrary.Conv_IntToDouble` (mod _current_point_index _theta_samples)) (`KismetMathLibrary.Conv_IntToDouble` (- (`self.phi_samples`) (/ _current_point_index _theta_samples)))))
  (while (and (<= (`self.phi`) 90.0) (<= (`local.iterator_l`) (`self.max_samples_per_frame`)) (<= (`self.current_point_index`) (`self.nb_points`)))
    (`|ExecutionSequence`
      (:`then_0`
        (if (and (`KismetArrayLibrary.Array_IsEmpty` _updatebox) (not (`self.IsFirstScan`)))
          (set `self.current_point_index` (`self.nb_points`))
          (else
            (for _array_element _updatebox
              (bind (_x _y _z _w) (`KismetMathLibrary.BreakVector4` _array_element))
              (set `local.should_update_l` (or (and (and (>= _returnvalue_3 _x) (<= _returnvalue_3 _z)) (and (>= _returnvalue_2 _y) (<= _returnvalue_2 _w))) (`local.should_update_l`)))))))
      (:`then_1`
        (if (or (`self.IsFirstScan`) (`local.should_update_l`))
          (bind _outhit (`KismetSystemLibrary.LineTraceSingle` :`Start` _returnvalue :`End` (+ _returnvalue (* (`self.PhiTheta2Vector` (`self.phi`) (`self.theta`)) 1500.0)) :`TraceChannel` "TraceTypeQuery1" :`DrawDebugType` "ForOneFrame"))
          (bind (_canvas _size _context) (`KismetRenderingLibrary.BeginDrawCanvasToRenderTarget` (`self.Point Cloud Texture`)))
          (`Canvas.K2_DrawLine` _canvas _returnvalue_4 (+ _returnvalue_4 (1.0 0.0)) 1.0 (make `LinearColor` (.x (`.ImpactPoint` (`GameplayStatics.BreakHitResult` _outhit))) (.y (`.ImpactPoint` (`GameplayStatics.BreakHitResult` _outhit))) (.z (`.ImpactPoint` (`GameplayStatics.BreakHitResult` _outhit)))))
          (`KismetRenderingLibrary.EndDrawCanvasToRenderTarget` _context)
          (`/Engine/EditorBlueprintResources/StandardMacros.IncrementInt` (`local.iterator_l`))))
      (:`then_2`
        (set `local.should_update_l` false)
        (bind _result (`/Engine/EditorBlueprintResources/StandardMacros.IncrementInt` (`self.current_point_index`))
          (:`  `
            (if (== (mod _result (`self.theta_samples`)) 0)
              (set `self.phi` (+ (`self.phi`) (`self.phi_step`)))
              (set `self.theta` -90.0)
              (else
                (set `self.theta` (+ (`self.theta`) (`self.theta_step`)))))))))))

(fn `UserConstructionScript`)