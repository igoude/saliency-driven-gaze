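; Bakes a PLY point cloud file into two square render targets: a point data texture and a saliency map.
; BeginPlay loads the named file from Content/PointClouds and sizes both targets from the square root of the point count.
; Tick decodes capped batches of points, drawing each as a one-pixel line in the data target and its alpha in the saliency target.
; Setting SaveMaps exports both maps as EXRs to hard-coded paths.
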(event `self.ReceiveBeginPlay`
  (bind _returnvalue (`CsvFileHelper.LoadPointCloudPlyFile` (`KismetSystemLibrary.GetProjectDirectory`) (`KismetStringLibrary.Concat_StrStr` "Content/PointClouds/" (`self.PlyFileName`) ".ply") (`self.PlyJson`)))
  (if (> _returnvalue 0)
    (bind _output_get (set `self.Nb Points in Cloud` _returnvalue))
    (bind _output_get_2 (set `self.Texture Size` (`KismetMathLibrary.FCeil` (`KismetMathLibrary.Sqrt` (`KismetMathLibrary.Conv_IntToDouble` _output_get)))))
    (bind _returnvalue_2 (`KismetRenderingLibrary.CreateRenderTarget2D` _output_get_2 _output_get_2 "RTF_RGBA16f" (struct)))
    (set `self.PointCloudTexture` _returnvalue_2)
    (bind _returnvalue_3 (`KismetRenderingLibrary.CreateRenderTarget2D` _output_get_2 _output_get_2 "RTF_RGBA16f" (struct)))
    (set `self.PointCloudSaliency` _returnvalue_3)
    (else
      (`KismetSystemLibrary.PrintString` "Unable to load ply file"))))

(event `self.ReceiveTick`
  (params (DeltaSeconds :type "Float (single-precision)"))
  (bind _current_point_index (`self.Current Point Index`))
  (bind _texture_size (`self.Texture Size`))
  (bind _returnvalue (< (`self.Current Point Index`) (`self.Nb Points in Cloud`)))
  (bind _returnvalue_2 (`KismetMathLibrary.MakeVector2D` (`KismetMathLibrary.Conv_IntToDouble` (mod _current_point_index _texture_size)) (`KismetMathLibrary.Conv_IntToDouble` (/ _current_point_index _texture_size))))
  (bind _returnvalue_3 (+ _returnvalue_2 (1.0 0.0)))
  (`|ExecutionSequence`
    (:`then_0`
      (if _returnvalue
        (bind _returnvalue_4 (`CsvFileHelper.LoadPointsJson` (`self.PlyJson`) (`self.Nb Points Max Per Frame`)))
        (for _array_element _returnvalue_4
          (`|ExecutionSequence`
            (:`then_0`
              (bind (_canvas _size _context) (`KismetRenderingLibrary.BeginDrawCanvasToRenderTarget` (`self.PointCloudTexture`)))
              (`Canvas.K2_DrawLine` _canvas _returnvalue_2 _returnvalue_3 1.0 _array_element)
              (`KismetRenderingLibrary.EndDrawCanvasToRenderTarget` _context))
            (:`then_1`
              (bind (_canvas_2 _size_2 _context_2) (`KismetRenderingLibrary.BeginDrawCanvasToRenderTarget` (`self.PointCloudSaliency`)))
              (bind (_r _g _b _a) (break `LinearColor` _array_element))
              (`Canvas.K2_DrawLine` _canvas_2 _returnvalue_2 _returnvalue_3 1.0 (make `LinearColor` _a _a _a _a))
              (`KismetRenderingLibrary.EndDrawCanvasToRenderTarget` _context_2))
            (:`then_2`
              (`/Engine/EditorBlueprintResources/StandardMacros.IncrementInt` (`self.Current Point Index`)))
            (:`then_3`
              (if (not _returnvalue)
                (break)))))))
    (:`then_1`
      (if (`self.Save Maps`)
        (set `self.Save Maps` false)
        (`ImageWriteBlueprintLibrary.ExportToDisk` (`self.PointCloudTexture`) "C:\\Users\\igoude\\Documents\\Unreal Projects\\UE5_Test_XP\\Content\\Textures\\Level_1_PC.exr" (make `ImageWriteOptions` "EXR" (delegate `ExportToDiskCompleteEvent`) 1))
        (`ImageWriteBlueprintLibrary.ExportToDisk` (`self.PointCloudSaliency`) "C:\\Users\\igoude\\Documents\\Unreal Projects\\UE5_Test_XP\\Content\\Textures\\Level_1_S.exr" (make `ImageWriteOptions` "EXR" (delegate `ExportToDiskCompleteEvent`) 1))))))

(event `ExportToDiskCompleteEvent`
  (params (bSuccess :type Boolean))
  (`KismetSystemLibrary.PrintString` "Texture successfully exported"))

(fn `UserConstructionScript`)