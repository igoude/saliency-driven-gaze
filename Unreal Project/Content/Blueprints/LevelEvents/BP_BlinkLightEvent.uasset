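; Level event that turns a light red and makes it blink erratically while steering a MetaHuman's gaze behavior toward it.
; Tick fires the event once game time passes a hardcoded threshold, then adjusts the gaze component's bias and saliency weights and sets the light as the focus task's target.
; Once triggered, each frame has a random chance to toggle the light between off and the intensity cached at BeginPlay.
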(event `self.ReceiveBeginPlay`
  (set `self.LightIntensity` (`LightComponentBase.Intensity` (`Light.LightComponent` (`self.Light`)))))

(event `self.OnEventTrigger`
  (bind _lightcomponent (`Light.LightComponent` (`self.Light`)))
  (set `self.IsTriggered` true)
  (`LightComponent.SetLightColor` _lightcomponent (struct :`R` 1.0 :`A` 1.0) true)
  (`LightComponent.SetIntensity` _lightcomponent 0.0)
  (set `self.OnOff` false))

(event `self.ReceiveTick`
  (params (DeltaSeconds :type "Float (single-precision)"))
  (bind _focustask (`self.FocusTask`))
  (bind _lightcomponent (`Light.LightComponent` (`self.Light`)))
  (bind _output (`|GetArrayItem` (`self.K2_GetComponentsByClass` (`self.Metahuman`) "/Game/Blueprints/Gaze/BP_MetaHumansGaze.BP_MetaHumansGaze_C")))
  (`|ExecutionSequence`
    (:`then_0`
      (if (`self.IsTriggered`)
        (if (< (`KismetMathLibrary.RandomFloat`) (`self.BlinkProbability`))
          (if (`self.OnOff`)
            (`LightComponent.SetIntensity` _lightcomponent 0.0)
            (set `self.OnOff` false)
            (else
              (`LightComponent.SetIntensity` _lightcomponent (`self.LightIntensity`))
              (set `self.OnOff` true))))))
    (:`then_1`
      (if (> (`GameplayStatics.GetTimeSeconds`) 25.0)
        (if (not (`self.IsTriggered`))
          (`self.OnEventTrigger`)
          (set `/Game/Blueprints/Gaze/BP_MetaHumansGaze.BiasWeight` 0.9 _output)
          (set `/Game/Blueprints/Gaze/BP_MetaHumansGaze.SaliencyWeight` 0.25 _output)
          (set `/Game/Blueprints/BiasMaps/BP_FocusTaskMap.FocusActor` (`self.Light`) _focustask)
          (set `/Game/Blueprints/BiasMaps/BP_FocusTaskMap.FocusSize` 0.15 _focustask))))))

(fn `UserConstructionScript`
  (`parent.UserConstructionScript`))