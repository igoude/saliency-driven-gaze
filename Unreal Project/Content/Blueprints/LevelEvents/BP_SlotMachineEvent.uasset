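; Slot machine level event that brightens a point light and spews randomly colored poker chips once triggered.
; Tick triggers it once when Happened is set and game time passes 25 seconds, also retuning a MetaHuman's gaze bias and saliency weights.
; While triggered, Tick ramps light intensity to a cap and randomly spawns red, green or blue chips, applying force within a forward cone.
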(event `self.OnEventTrigger`
  (set `self.IsTriggered` true)
  (set `self.StartEventTime` (`GameplayStatics.GetTimeSeconds`)))

(event `self.ReceiveTick`
  (params (DeltaSeconds :type "Float (single-precision)"))
  (bind _returnvalue (`KismetMathLibrary.RandomFloat`))
  (bind _returnvalue_2 (`KismetMathLibrary.RandomUnitVectorInConeInDegrees` (`self.GetActorForwardVector`) 15.0))
  (bind _output (`|GetArrayItem` (`self.K2_GetComponentsByClass` (`self.Metahuman`) "/Game/Blueprints/Gaze/BP_MetaHumansGaze.BP_MetaHumansGaze_C")))
  (bind _intensity (`LightComponentBase.Intensity` (`PointLight.PointLightComponent` (`self.Light`))))
  (bind _returnvalue_3 (`KismetMathLibrary.MakeTransform` (+ (`self.K2_GetActorLocation`) (* (`KismetMathLibrary.RandomUnitVector`) (`KismetMathLibrary.RandomFloat`))) (`KismetMathLibrary.RandomRotator` false)))
  (`|ExecutionSequence`
    (:`then_0`
      (if (`self.IsTriggered`)
        (`|ExecutionSequence`
          (:`then_0`
            (if (<= _intensity 10.0)
              (`LightComponent.SetIntensity` (`PointLight.PointLightComponent` (`self.Light`)) (+ _intensity 0.1))))
          (:`then_1`
            (if (< (`KismetMathLibrary.RandomFloat`) (`self.SpawnProbability`))
              (if (< _returnvalue 0.33)
                (bind _returnvalue_4 (`|SpawnActorFromClass` "/Game/Assets/Casino/low-poly-poker-chips-cards/PokerChipRed_BP.PokerChipRed_BP_C" _returnvalue_3 "Undefined" "OverrideRootScale" null null))
                (`PrimitiveComponent.AddForce` (`StaticMeshActor.StaticMeshComponent` _returnvalue_4) _returnvalue_2 "None" false)
                (elif (< _returnvalue 0.66)
                  (bind _returnvalue_5 (`|SpawnActorFromClass` "/Game/Assets/Casino/low-poly-poker-chips-cards/PokerChipGreen_BP.PokerChipGreen_BP_C" _returnvalue_3 "Undefined" "OverrideRootScale" null null))
                  (`PrimitiveComponent.AddForce` (`StaticMeshActor.StaticMeshComponent` _returnvalue_5) _returnvalue_2 "None" false)
                  (else
                    (bind _returnvalue_6 (`|SpawnActorFromClass` "/Game/Assets/Casino/low-poly-poker-chips-cards/PokerChipBlue_BP.PokerChipBlue_BP_C" _returnvalue_3 "Undefined" "OverrideRootScale" null null))
                    (`PrimitiveComponent.AddForce` (`StaticMeshActor.StaticMeshComponent` _returnvalue_6) _returnvalue_2 "None" false)))))))))
    (:`then_1`
      (if (`self.Happened`)
        (if (> (`GameplayStatics.GetTimeSeconds`) 25.0)
          (if (not (`self.IsTriggered`))
            (`self.OnEventTrigger`)
            (set `/Game/Blueprints/Gaze/BP_MetaHumansGaze.BiasWeight` 0.9 _output)
            (set `/Game/Blueprints/Gaze/BP_MetaHumansGaze.SaliencyWeight` 0.25 _output)))))))

(fn `UserConstructionScript`
  (`parent.UserConstructionScript`))