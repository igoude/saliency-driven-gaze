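; Level event that stages a MetaHuman opening a door, with a spotlight brightening as it opens and dimming as it closes.
; Once game time passes a fixed delay, Tick triggers the character's AnimBP and retunes a viewer MetaHuman's gaze bias and saliency weights.
; Boolean phases timed from animation start then drive door yaw and light intensity in fixed per-frame steps, without delta-time scaling.
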(event `self.OnEventTrigger`
  (set `self.IsTriggered` true)
  (bind _asopen_door_idle_anim_bp (cast `/Game/MH/Animation/OpenDoor_Idle_AnimBP` (`SkeletalMeshComponent.GetAnimInstance` (`|GetArrayItem` (`self.GetComponentsByTag` (`self.Metahuman`) "/Script/Engine.SkeletalMeshComponent" "MetaHumanBody")))))
  (bind _output_get (set `self.AnimBP` _asopen_door_idle_anim_bp))
  (`/Game/MH/Animation/OpenDoor_Idle_AnimBP.OpenDoorStart` _output_get)
  (set `self.StartTimeAnim` (`GameplayStatics.GetTimeSeconds`))
  (set `self.WaitingForAnimationStart` true))

(event `self.ReceiveTick`
  (params (DeltaSeconds :type "Float (single-precision)"))
  (bind _dooractor (`self.DoorActor`))
  (bind _dooractor_2 (`self.DoorActor`))
  (bind (_returnvalue_roll _returnvalue_pitch _returnvalue_yaw) (`KismetMathLibrary.BreakRotator` (`self.K2_GetActorRotation` _dooractor)))
  (bind (_returnvalue_roll_2 _returnvalue_pitch_2 _returnvalue_yaw_2) (`KismetMathLibrary.BreakRotator` (`self.K2_GetActorRotation` _dooractor_2)))
  (bind _returnvalue (<= (`self.CurrentIntensity`) 32.0))
  (bind _returnvalue_2 (>= (`self.CurrentIntensity`) 0.0))
  (bind _output (`|GetArrayItem` (`self.K2_GetComponentsByClass` (`self.Metahuman_Viewer`) "/Game/Blueprints/Gaze/BP_MetaHumansGaze.BP_MetaHumansGaze_C")))
  (bind _returnvalue_3 (<= _returnvalue_yaw_2 130.0))
  (bind _returnvalue_4 (>= _returnvalue_yaw 90.0))
  (`|ExecutionSequence`
    (:`then_0`
      (if (`self.WaitingForAnimationStart`)
        (if (> (- (`GameplayStatics.GetTimeSeconds`) (`self.StartTimeAnim`)) (`self.StartOpeningTime`))
          (set `self.WaitingForAnimationStart` false)
          (set `self.OpeningDoor` true))))
    (:`then_1`
      (if (`self.OpeningDoor`)
        (`|ExecutionSequence`
          (:`then_0`
            (if _returnvalue_3
              (`self.K2_AddActorLocalRotation` _dooractor_2 (`KismetMathLibrary.MakeRotator` 0.0 0.0 (`self.DoorSpeed`)) false false)))
          (:`then_1`
            (if _returnvalue
              (bind _output_get (set `self.CurrentIntensity` (+ (`self.CurrentIntensity`) (`self.LightSpeed`))))
              (`LightComponent.SetIntensity` (`SpotLight.SpotLightComponent` (`self.Light`)) _output_get)))
          (:`then_2`
            (if (`KismetMathLibrary.BooleanNOR` _returnvalue_3 _returnvalue)
              (set `self.OpeningDoor` false)
              (set `self.WaitingForAnimationIdle` true))))))
    (:`then_2`
      (if (`self.WaitingForAnimationIdle`)
        (if (> (- (`GameplayStatics.GetTimeSeconds`) (`self.StartTimeAnim`)) (`self.StartClosingTime`))
          (set `self.WaitingForAnimationIdle` false)
          (set `self.ClosingDoor` true))))
    (:`then_3`
      (if (`self.ClosingDoor`)
        (`|ExecutionSequence`
          (:`then_0`
            (if _returnvalue_4
              (`self.K2_AddActorLocalRotation` _dooractor (`KismetMathLibrary.MakeRotator` 0.0 0.0 (- 0.0 (`self.DoorSpeed`))) false false)))
          (:`then_1`
            (if _returnvalue_2
              (bind _output_get_2 (set `self.CurrentIntensity` (- (`self.CurrentIntensity`) (`self.LightSpeed`))))
              (`LightComponent.SetIntensity` (`SpotLight.SpotLightComponent` (`self.Light`)) _output_get_2)))
          (:`then_2`
            (if (`KismetMathLibrary.BooleanNOR` _returnvalue_4 _returnvalue_2)
              (set `self.ClosingDoor` false))))))
    (:`then_4`
      (if (> (`GameplayStatics.GetTimeSeconds`) 14.0)
        (if (not (`self.IsTriggered`))
          (`self.OnEventTrigger`)
          (set `/Game/Blueprints/Gaze/BP_MetaHumansGaze.BiasWeight` 0.9 _output)
          (set `/Game/Blueprints/Gaze/BP_MetaHumansGaze.SaliencyWeight` 0.25 _output))))))

(fn `UserConstructionScript`
  (`parent.UserConstructionScript`))