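; BP_FixationTable is an actor that records gaze fixations and reads them back from a data table.
; AddFixation appends to an array, which SaveFixationTable writes as an overwritable CSV under the project's Content/Tables/MetaGaze folder.
; Separately, LoadFixationTable assigns a data table, and GetFixation returns rows sequentially by index-based row name, advancing the index only when a row is found.
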(fn `AddFixation`
  (params (Fixation :type "FixationData Structure"))
  (`KismetArrayLibrary.Array_Add` (`self.FixationArray`) Fixation))

(fn `GetFixation`
  (returns (Fixation :type "FixationData Structure") (Found :type Boolean))
  (locals (CurrentFixation :type " Structure"))
  (bind _returnvalue (`|GetDataTableRow` (`self.FixationTable`) (`KismetStringLibrary.Conv_StringToName` (`KismetStringLibrary.Conv_IntToString` (`self.CurrentIndex`))))
    (:`then`
      (`/Engine/EditorBlueprintResources/StandardMacros.IncrementInt` (`self.CurrentIndex`)
        (:`  `
          (return _returnvalue true))))
    (:`RowNotFound`
      (return (struct) false))))

(fn `LoadFixationTable`
  (params (DataTable :type "DataTable Object Reference"))
  (set `self.FixationTable` DataTable))

(fn `SaveFixationTable`
  (params (Filename :type String))
  (`CsvFileHelper.SaveFixationTableToCsvFile` (`KismetSystemLibrary.GetProjectDirectory`) (`KismetStringLibrary.Concat_StrStr` "Content/Tables/MetaGaze/" Filename ".csv") (`self.FixationArray`) true))

(fn `UserConstructionScript`)