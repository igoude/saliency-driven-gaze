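; BP_SalientPointActor is a gaze target that tracks how inhibited it is from being fixated.
; On BeginPlay it draws its fixation duration from a gamma distribution.
; Exposed functions raise a fixation timer by delta time or lower it scaled by InhibitionSpeed, and inhibition is that timer divided by the duration.
; Each Tick scales the sphere by the inhibition value as a visual indicator.
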(event `self.ReceiveBeginPlay`
  (bind _returnvalue (`NormalRandom.GammaRandom` 1.239396 0.080006 0.188045))
  (set `self.FixationDuration` _returnvalue))

(event `self.ReceiveTick`
  (params (DeltaSeconds :type "Float (single-precision)"))
  (bind _inhibitionvalue (`self.GetInhibitionValue`))
  (`SceneComponent.SetWorldScale3D` (`self.Sphere`) (`KismetMathLibrary.Conv_DoubleToVector` (* _inhibitionvalue 0.1))))

(fn `DecreaseTimer`
  (params (deltaTime :type "Float (double-precision)"))
  (set `self.FixationTimer` (- (`self.FixationTimer`) (* deltaTime (`self.InhibitionSpeed`)))))

(fn `GetInhibitionValue`
  (returns (InhibitionValue :type "Float (double-precision)"))
  (if (> (`self.FixationDuration`) 0.0)
    (return (/ (`self.FixationTimer`) (`self.FixationDuration`)))
    (else
      (return 0.0))))

(fn `IncreaseTimer`
  (params (deltaTime :type "Float (double-precision)"))
  (set `self.FixationTimer` (+ deltaTime (`self.FixationTimer`))))

(fn `UserConstructionScript`)