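; BP_FocusBiasMap is a bias map actor that renders a single-point focus task map for a MetaHuman gaze system, centered on a focus actor.
; BeginPlay creates a dynamic instance of M_OnePointFocusMaterial.
; RenderTaskMap converts the FocusActor's world location into the gaze's eye-camera space, feeds that position and FocusSize into the material, then draws it to the TaskMap render target.
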(event `self.ReceiveBeginPlay`
  (`parent.ReceiveBeginPlay`)
  (bind _returnvalue (`KismetMaterialLibrary.CreateDynamicMaterialInstance` "/Game/Materials/Biases/M_OnePointFocusMaterial.M_OnePointFocusMaterial"))
  (set `self.TaskMaterial` _returnvalue))

(fn `RenderTaskMap`
  (params (MetaHumanGaze :type "/Game/Blueprints/Gaze/BP_MetaHumansGaze Object Reference"))
  (bind _taskmaterial (`self.TaskMaterial`))
  (bind _uv_coordinate (`/Game/Blueprints/Gaze/BP_MetaHumansGaze.WorldToEyeCameraTransform` MetaHumanGaze (`self.K2_GetActorLocation` (`self.FocusActor`))))
  (`MaterialInstanceDynamic.SetVectorParameterValue` _taskmaterial "uv" (make `LinearColor` (`KismetMathLibrary.BreakVector2D` _uv_coordinate) (`.Y` (`KismetMathLibrary.BreakVector2D` _uv_coordinate))))
  (`MaterialInstanceDynamic.SetScalarParameterValue` _taskmaterial "Size" (`self.FocusSize`))
  (`KismetRenderingLibrary.DrawMaterialToRenderTarget` (`self.TaskMap`) _taskmaterial))

(fn `UserConstructionScript`
  (`parent.UserConstructionScript`))