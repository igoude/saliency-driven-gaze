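; Idle bias map Blueprint that renders a task map for a MetaHuman gaze system, based on the current eye direction.
; On BeginPlay it creates a dynamic instance of M_IdleBiasMaterial.
; RenderTaskMap converts the left eye socket's rotation into body space and remaps yaw and pitch to normalized UV coordinates.
; It passes these to the material's "uv" parameter, then draws the material into the TaskMap render target.
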(event `self.ReceiveBeginPlay`
  (`parent.ReceiveBeginPlay`)
  (bind _returnvalue (`KismetMaterialLibrary.CreateDynamicMaterialInstance` "/Game/Materials/Biases/M_IdleBiasMaterial.M_IdleBiasMaterial"))
  (set `self.TaskMaterial` _returnvalue))

(fn `RenderTaskMap`
  (params (MetaHumanGaze :type "/Game/Blueprints/Gaze/BP_MetaHumansGaze Object Reference"))
  (bind _taskmaterial (`self.TaskMaterial`))
  (`MaterialInstanceDynamic.SetVectorParameterValue` _taskmaterial "uv" (make `LinearColor` (/ (+ (/ (- (.yaw (`KismetMathLibrary.InverseTransformRotation` (`SceneComponent.K2_GetComponentToWorld` (`/Game/Blueprints/Gaze/BP_MetaHumansGaze.MetaHumanBody` MetaHumanGaze)) (`SceneComponent.GetSocketRotation` (`/Game/Blueprints/Gaze/BP_MetaHumansGaze.MetaHumanFace` MetaHumanGaze) "Eye_L_Socket"))) 90.0) 90.0) 1.0) 2.0) (/ (+ (/ (.pitch (`KismetMathLibrary.InverseTransformRotation` (`SceneComponent.K2_GetComponentToWorld` (`/Game/Blueprints/Gaze/BP_MetaHumansGaze.MetaHumanBody` MetaHumanGaze)) (`SceneComponent.GetSocketRotation` (`/Game/Blueprints/Gaze/BP_MetaHumansGaze.MetaHumanFace` MetaHumanGaze) "Eye_L_Socket"))) 45.0) 1.0) 2.0)))
  (`KismetRenderingLibrary.DrawMaterialToRenderTarget` (`self.TaskMap`) _taskmaterial))

(fn `UserConstructionScript`
  (`parent.UserConstructionScript`))