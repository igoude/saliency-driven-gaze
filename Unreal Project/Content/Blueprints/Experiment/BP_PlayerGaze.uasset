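; BP_PlayerGaze records and visualizes the player's eye-tracking gaze during experiment levels.
; Each tick, DebugGaze moves a sphere to the fixation point, while RecordGaze logs fixation, head pose and per-eye gaze to BP_FixationTable.
; Left, right and combined gaze directions become 2D coordinates through a synthetic fixed-FOV view-projection.
; EndPlay saves the table under UserGaze by level and user ID, adding LevelCounter for the "Loby" level.
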(event `self.ReceiveBeginPlay`
  (bind _asbp_experiment_instance (cast `/Game/Blueprints/GameMode/BP_ExperimentInstance` (`GameplayStatics.GetGameInstance`)))
  (set `self.As BP Experiment Instance` _asbp_experiment_instance)
  (if (`self.RecordGaze`)
    (bind _returnvalue (`GameplayStatics.GetActorOfClass` "/Game/Blueprints/Gaze/BP_FixationTable.BP_FixationTable_C"))
    (set `self.FixationTable` _returnvalue)))

(event `self.ReceiveEndPlay`
  (params (EndPlayReason :type "EEndPlayReason Enum" :default "Destroyed"))
  (bind _fixationtable (`self.FixationTable`))
  (if (`self.RecordGaze`)
    (bind _returnvalue (`GameplayStatics.GetCurrentLevelName` true))
    (bind _asbp_experiment_instance (cast `/Game/Blueprints/GameMode/BP_ExperimentInstance` (`GameplayStatics.GetGameInstance`)))
    (if (== _returnvalue "Loby")
      (bind _returnvalue_2 (`KismetStringLibrary.Conv_NameToString` (`/Game/Blueprints/GameMode/BP_ExperimentInstance.UserID` _asbp_experiment_instance)))
      (`/Game/Blueprints/Gaze/BP_FixationTable.SaveFixationTable` _fixationtable (`KismetStringLibrary.Concat_StrStr` "UserGaze/" _returnvalue "_" (`KismetStringLibrary.Conv_IntToString` (`/Game/Blueprints/GameMode/BP_ExperimentInstance.LevelCounter` _asbp_experiment_instance)) "_" _returnvalue_2))
      (else
        (`/Game/Blueprints/Gaze/BP_FixationTable.SaveFixationTable` _fixationtable (`KismetStringLibrary.Concat_StrStr` "UserGaze/" _returnvalue "_" _returnvalue_2))))))

(event `self.ReceiveTick`
  (params (DeltaSeconds :type "Float (single-precision)"))
  (bind _returnvalue (`GameplayStatics.GetPlayerCameraManager` 0))
  (if (or (`self.RecordGaze`) (`self.DebugGaze`))
    (bind _outgazedata (`EyeTrackerFunctionLibrary.GetGazeData`))
    (`|ExecutionSequence`
      (:`then_0`
        (if (`self.DebugGaze`)
          (bind (_gazeorigin _gazedirection _fixationpoint) (break `EyeTrackerGazeData` _outgazedata))
          (`SceneComponent.K2_SetWorldLocation` (`self.Sphere`) _fixationpoint false true)))
      (:`then_1`
        (if (`self.RecordGaze`)
          (bind _outgazedata_2 (`EyeTrackerFunctionLibrary.GetStereoGazeData`))
          (bind (_lefteyeorigin _lefteyedirection _righteyeorigin _righteyedirection) (break `EyeTrackerStereoGazeData` _outgazedata_2))
          (bind (_returnvalue_x _returnvalue_y _returnvalue_z _returnvalue_w) (`KismetMathLibrary.BreakVector4` (`KismetMathLibrary.Matrix_TransformVector` (`.ViewProjectionMatrix` (`GameplayStatics.GetViewProjectionMatrix` (make `MinimalViewInfo` _lefteyeorigin (struct) 110.0 512.0 0.0 2097152.0 1.0 true false "Perspective" 0.0 (struct :`BloomMethod` "BM_SOG" :`AutoExposureMethod` "AEM_Histogram" :`TemperatureType` "TEMP_WhiteBalance" :`WhiteTemp` 6500.0 :`ColorSaturation` (struct :`X` 1.0 :`Y` 1.0 :`Z` 1.0 :`W` 1.0) :`ColorContrast` (struct :`X` 1.0 :`Y` 1.0 :`Z` 1.0 :`W` 1.0) :`ColorGamma` (struct :`X` 1.0 :`Y` 1.0 :`Z` 1.0 :`W` 1.0) :`ColorGain` (struct :`X` 1.0 :`Y` 1.0 :`Z` 1.0 :`W` 1.0) :`ColorOffset` (struct) :`ColorSaturationShadows` (struct :`X` 1.0 :`Y` 1.0 :`Z` 1.0 :`W` 1.0) :`ColorContrastShadows` (struct :`X` 1.0 :`Y` 1.0 :`Z` 1.0 :`W` 1.0) :`ColorGammaShadows` (struct :`X` 1.0 :`Y` 1.0 :`Z` 1.0 :`W` 1.0) :`ColorGainShadows` (struct :`X` 1.0 :`Y` 1.0 :`Z` 1.0 :`W` 1.0) :`ColorOffsetShadows` (struct) :`ColorSaturationMidtones` (struct :`X` 1.0 :`Y` 1.0 :`Z` 1.0 :`W` 1.0) :`ColorContrastMidtones` (struct :`X` 1.0 :`Y` 1.0 :`Z` 1.0 :`W` 1.0) :`ColorGammaMidtones` (struct :`X` 1.0 :`Y` 1.0 :`Z` 1.0 :`W` 1.0) :`ColorGainMidtones` (struct :`X` 1.0 :`Y` 1.0 :`Z` 1.0 :`W` 1.0) :`ColorOffsetMidtones` (struct) :`ColorSaturationHighlights` (struct :`X` 1.0 :`Y` 1.0 :`Z` 1.0 :`W` 1.0) :`ColorContrastHighlights` (struct :`X` 1.0 :`Y` 1.0 :`Z` 1.0 :`W` 1.0) :`ColorGammaHighlights` (struct :`X` 1.0 :`Y` 1.0 :`Z` 1.0 :`W` 1.0) :`ColorGainHighlights` (struct :`X` 1.0 :`Y` 1.0 :`Z` 1.0 :`W` 1.0) :`ColorOffsetHighlights` (struct) :`ColorCorrectionHighlightsMin` 0.5 :`ColorCorrectionHighlightsMax` 1.0 :`ColorCorrectionShadowsMax` 0.09 :`BlueCorrection` 0.6 :`ExpandGamut` 1.0 :`ToneCurveAmount` 1.0 :`FilmSlope` 0.88 :`FilmToe` 0.55 :`FilmShoulder` 0.26 :`FilmWhiteClip` 0.04 :`SceneColorTint` (struct :`R` 1.0 :`G` 1.0 :`B` 1.0 :`A` 1.0) :`BloomIntensity` 0.675 :`BloomThreshold` -1.0 :`BloomSizeScale` 4.0 :`Bloom1Size` 0.3 :`Bloom2Size` 1.0 :`Bloom3Size` 2.0 :`Bloom4Size` 10.0 :`Bloom5Size` 30.0 :`Bloom6Size` 64.0 :`Bloom1Tint` (struct :`R` 0.3465 :`G` 0.3465 :`B` 0.3465 :`A` 1.0) :`Bloom2Tint` (struct :`R` 0.138 :`G` 0.138 :`B` 0.138 :`A` 1.0) :`Bloom3Tint` (struct :`R` 0.1176 :`G` 0.1176 :`B` 0.1176 :`A` 1.0) :`Bloom4Tint` (struct :`R` 0.066 :`G` 0.066 :`B` 0.066 :`A` 1.0) :`Bloom5Tint` (struct :`R` 0.066 :`G` 0.066 :`B` 0.066 :`A` 1.0) :`Bloom6Tint` (struct :`R` 0.061 :`G` 0.061 :`B` 0.061 :`A` 1.0) :`BloomConvolutionScatterDispersion` 1.0 :`BloomConvolutionSize` 1.0 :`BloomConvolutionCenterUV` (0.5 0.5) :`BloomConvolutionPreFilterMin` 7.0 :`BloomConvolutionPreFilterMax` 15000.0 :`BloomConvolutionPreFilterMult` 15.0 :`BloomConvolutionBufferScale` 0.133 :`BloomDirtMaskTint` (struct :`R` 0.5 :`G` 0.5 :`B` 0.5 :`A` 1.0) :`DynamicGlobalIlluminationMethod` "Lumen" :`IndirectLightingColor` (struct :`R` 1.0 :`G` 1.0 :`B` 1.0 :`A` 1.0) :`IndirectLightingIntensity` 1.0 :`LumenSceneLightingQuality` 1.0 :`LumenSceneDetail` 1.0 :`LumenSceneViewDistance` 20000.0 :`LumenSceneLightingUpdateSpeed` 1.0 :`LumenFinalGatherQuality` 1.0 :`LumenFinalGatherLightingUpdateSpeed` 1.0 :`LumenMaxTraceDistance` 20000.0 :`RayTracingGIType` "Disabled" :`RayTracingGIMaxBounces` 1 :`RayTracingGISamplesPerPixel` 4 :`ReflectionMethod` "Lumen" :`LumenReflectionQuality` 1.0 :`LumenRayLightingMode` "Default" :`ScreenSpaceReflectionIntensity` 100.0 :`ScreenSpaceReflectionQuality` 50.0 :`ScreenSpaceReflectionMaxRoughness` 0.6 :`RayTracingReflectionsMaxRoughness` 0.6 :`RayTracingReflectionsMaxBounces` 1 :`RayTracingReflectionsSamplesPerPixel` 1 :`RayTracingReflectionsShadows` "Hard_shadows" :`AmbientCubemapTint` (struct :`R` 1.0 :`G` 1.0 :`B` 1.0 :`A` 1.0) :`AmbientCubemapIntensity` 1.0 :`CameraShutterSpeed` 60.0 :`CameraISO` 100.0 :`DepthOfFieldFstop` 4.0 :`DepthOfFieldMinFstop` 1.2 :`DepthOfFieldBladeCount` 5 :`AutoExposureBias` 1.0 :`AutoExposureApplyPhysicalCameraExposure` true :`AutoExposureLowPercent` 10.0 :`AutoExposureHighPercent` 90.0 :`AutoExposureMinBrightness` -10.0 :`AutoExposureMaxBrightness` 20.0 :`AutoExposureSpeedUp` 3.0 :`AutoExposureSpeedDown` 1.0 :`HistogramLogMin` -10.0 :`HistogramLogMax` 20.0 :`LocalExposureContrastScale` 1.0 :`LocalExposureDetailStrength` 1.0 :`LocalExposureBlurredLuminanceBlend` 0.6 :`LocalExposureBlurredLuminanceKernelSizePercent` 50.0 :`LensFlareIntensity` 1.0 :`LensFlareTint` (struct :`R` 1.0 :`G` 1.0 :`B` 1.0 :`A` 1.0) :`LensFlareBokehSize` 3.0 :`LensFlareThreshold` 8.0 :`LensFlareTints[0]` (struct :`R` 1.0 :`G` 0.8 :`B` 0.4 :`A` 0.6) :`LensFlareTints[1]` (struct :`R` 1.0 :`G` 1.0 :`B` 0.6 :`A` 0.53) :`LensFlareTints[2]` (struct :`R` 0.8 :`G` 0.8 :`B` 1.0 :`A` 0.46) :`LensFlareTints[3]` (struct :`R` 0.5 :`G` 1.0 :`B` 0.4 :`A` 0.39) :`LensFlareTints[4]` (struct :`R` 0.5 :`G` 0.8 :`B` 1.0 :`A` 0.31) :`LensFlareTints[5]` (struct :`R` 0.9 :`G` 1.0 :`B` 0.8 :`A` 0.27) :`LensFlareTints[6]` (struct :`R` 1.0 :`G` 0.8 :`B` 0.4 :`A` 0.22) :`LensFlareTints[7]` (struct :`R` 0.9 :`G` 0.7 :`B` 0.7 :`A` 0.15) :`VignetteIntensity` 0.4 :`FilmGrainIntensityShadows` 1.0 :`FilmGrainIntensityMidtones` 1.0 :`FilmGrainIntensityHighlights` 1.0 :`FilmGrainShadowsMax` 0.09 :`FilmGrainHighlightsMin` 0.5 :`FilmGrainHighlightsMax` 1.0 :`FilmGrainTexelSize` 1.0 :`AmbientOcclusionIntensity` 0.5 :`AmbientOcclusionStaticFraction` 1.0 :`AmbientOcclusionRadius` 200.0 :`AmbientOcclusionFadeDistance` 8000.0 :`AmbientOcclusionFadeRadius` 5000.0 :`AmbientOcclusionPower` 2.0 :`AmbientOcclusionBias` 3.0 :`AmbientOcclusionQuality` 50.0 :`AmbientOcclusionMipBlend` 0.6 :`AmbientOcclusionMipScale` 1.7 :`AmbientOcclusionMipThreshold` 0.01 :`AmbientOcclusionTemporalBlendWeight` 0.1 :`RayTracingAO` true :`RayTracingAOSamplesPerPixel` 1 :`RayTracingAOIntensity` 1.0 :`RayTracingAORadius` 200.0 :`ColorGradingIntensity` 1.0 :`DepthOfFieldSensorWidth` 24.576 :`DepthOfFieldDepthBlurAmount` 1.0 :`DepthOfFieldNearTransitionRegion` 300.0 :`DepthOfFieldFarTransitionRegion` 500.0 :`DepthOfFieldNearBlurSize` 15.0 :`DepthOfFieldFarBlurSize` 15.0 :`DepthOfFieldOcclusion` 0.4 :`DepthOfFieldVignetteSize` 200.0 :`MotionBlurAmount` 0.5 :`MotionBlurMax` 5.0 :`MotionBlurTargetFPS` 30 :`MotionBlurPerObjectSize` 0.5 :`TranslucencyType` "Raster" :`RayTracingTranslucencyMaxRoughness` 0.6 :`RayTracingTranslucencyRefractionRays` 3 :`RayTracingTranslucencySamplesPerPixel` 1 :`RayTracingTranslucencyShadows` "Hard_shadows" :`RayTracingTranslucencyRefraction` true :`PathTracingMaxBounces` 32 :`PathTracingSamplesPerPixel` 16384 :`PathTracingFilterWidth` 3.0 :`PathTracingEnableEmissive` true :`PathTracingMaxPathExposure` 30.0 :`PathTracingEnableDenoiser` true :`WeightedBlendables` (struct))))) _lefteyedirection)))
          (bind (_returnvalue_x_2 _returnvalue_y_2 _returnvalue_z_2 _returnvalue_w_2) (`KismetMathLibrary.BreakVector4` (`KismetMathLibrary.Matrix_TransformVector` (`.ViewProjectionMatrix` (`GameplayStatics.GetViewProjectionMatrix` (make `MinimalViewInfo` _righteyeorigin (struct) 110.0 512.0 0.0 2097152.0 1.0 true false "Perspective" 0.0 (struct :`BloomMethod` "BM_SOG" :`AutoExposureMethod` "AEM_Histogram" :`TemperatureType` "TEMP_WhiteBalance" :`WhiteTemp` 6500.0 :`ColorSaturation` (struct :`X` 1.0 :`Y` 1.0 :`Z` 1.0 :`W` 1.0) :`ColorContrast` (struct :`X` 1.0 :`Y` 1.0 :`Z` 1.0 :`W` 1.0) :`ColorGamma` (struct :`X` 1.0 :`Y` 1.0 :`Z` 1.0 :`W` 1.0) :`ColorGain` (struct :`X` 1.0 :`Y` 1.0 :`Z` 1.0 :`W` 1.0) :`ColorOffset` (struct) :`ColorSaturationShadows` (struct :`X` 1.0 :`Y` 1.0 :`Z` 1.0 :`W` 1.0) :`ColorContrastShadows` (struct :`X` 1.0 :`Y` 1.0 :`Z` 1.0 :`W` 1.0) :`ColorGammaShadows` (struct :`X` 1.0 :`Y` 1.0 :`Z` 1.0 :`W` 1.0) :`ColorGainShadows` (struct :`X` 1.0 :`Y` 1.0 :`Z` 1.0 :`W` 1.0) :`ColorOffsetShadows` (struct) :`ColorSaturationMidtones` (struct :`X` 1.0 :`Y` 1.0 :`Z` 1.0 :`W` 1.0) :`ColorContrastMidtones` (struct :`X` 1.0 :`Y` 1.0 :`Z` 1.0 :`W` 1.0) :`ColorGammaMidtones` (struct :`X` 1.0 :`Y` 1.0 :`Z` 1.0 :`W` 1.0) :`ColorGainMidtones` (struct :`X` 1.0 :`Y` 1.0 :`Z` 1.0 :`W` 1.0) :`ColorOffsetMidtones` (struct) :`ColorSaturationHighlights` (struct :`X` 1.0 :`Y` 1.0 :`Z` 1.0 :`W` 1.0) :`ColorContrastHighlights` (struct :`X` 1.0 :`Y` 1.0 :`Z` 1.0 :`W` 1.0) :`ColorGammaHighlights` (struct :`X` 1.0 :`Y` 1.0 :`Z` 1.0 :`W` 1.0) :`ColorGainHighlights` (struct :`X` 1.0 :`Y` 1.0 :`Z` 1.0 :`W` 1.0) :`ColorOffsetHighlights` (struct) :`ColorCorrectionHighlightsMin` 0.5 :`ColorCorrectionHighlightsMax` 1.0 :`ColorCorrectionShadowsMax` 0.09 :`BlueCorrection` 0.6 :`ExpandGamut` 1.0 :`ToneCurveAmount` 1.0 :`FilmSlope` 0.88 :`FilmToe` 0.55 :`FilmShoulder` 0.26 :`FilmWhiteClip` 0.04 :`SceneColorTint` (struct :`R` 1.0 :`G` 1.0 :`B` 1.0 :`A` 1.0) :`BloomIntensity` 0.675 :`BloomThreshold` -1.0 :`BloomSizeScale` 4.0 :`Bloom1Size` 0.3 :`Bloom2Size` 1.0 :`Bloom3Size` 2.0 :`Bloom4Size` 10.0 :`Bloom5Size` 30.0 :`Bloom6Size` 64.0 :`Bloom1Tint` (struct :`R` 0.3465 :`G` 0.3465 :`B` 0.3465 :`A` 1.0) :`Bloom2Tint` (struct :`R` 0.138 :`G` 0.138 :`B` 0.138 :`A` 1.0) :`Bloom3Tint` (struct :`R` 0.1176 :`G` 0.1176 :`B` 0.1176 :`A` 1.0) :`Bloom4Tint` (struct :`R` 0.066 :`G` 0.066 :`B` 0.066 :`A` 1.0) :`Bloom5Tint` (struct :`R` 0.066 :`G` 0.066 :`B` 0.066 :`A` 1.0) :`Bloom6Tint` (struct :`R` 0.061 :`G` 0.061 :`B` 0.061 :`A` 1.0) :`BloomConvolutionScatterDispersion` 1.0 :`BloomConvolutionSize` 1.0 :`BloomConvolutionCenterUV` (0.5 0.5) :`BloomConvolutionPreFilterMin` 7.0 :`BloomConvolutionPreFilterMax` 15000.0 :`BloomConvolutionPreFilterMult` 15.0 :`BloomConvolutionBufferScale` 0.133 :`BloomDirtMaskTint` (struct :`R` 0.5 :`G` 0.5 :`B` 0.5 :`A` 1.0) :`DynamicGlobalIlluminationMethod` "Lumen" :`IndirectLightingColor` (struct :`R` 1.0 :`G` 1.0 :`B` 1.0 :`A` 1.0) :`IndirectLightingIntensity` 1.0 :`LumenSceneLightingQuality` 1.0 :`LumenSceneDetail` 1.0 :`LumenSceneViewDistance` 20000.0 :`LumenSceneLightingUpdateSpeed` 1.0 :`LumenFinalGatherQuality` 1.0 :`LumenFinalGatherLightingUpdateSpeed` 1.0 :`LumenMaxTraceDistance` 20000.0 :`RayTracingGIType` "Disabled" :`RayTracingGIMaxBounces` 1 :`RayTracingGISamplesPerPixel` 4 :`ReflectionMethod` "Lumen" :`LumenReflectionQuality` 1.0 :`LumenRayLightingMode` "Default" :`ScreenSpaceReflectionIntensity` 100.0 :`ScreenSpaceReflectionQuality` 50.0 :`ScreenSpaceReflectionMaxRoughness` 0.6 :`RayTracingReflectionsMaxRoughness` 0.6 :`RayTracingReflectionsMaxBounces` 1 :`RayTracingReflectionsSamplesPerPixel` 1 :`RayTracingReflectionsShadows` "Hard_shadows" :`AmbientCubemapTint` (struct :`R` 1.0 :`G` 1.0 :`B` 1.0 :`A` 1.0) :`AmbientCubemapIntensity` 1.0 :`CameraShutterSpeed` 60.0 :`CameraISO` 100.0 :`DepthOfFieldFstop` 4.0 :`DepthOfFieldMinFstop` 1.2 :`DepthOfFieldBladeCount` 5 :`AutoExposureBias` 1.0 :`AutoExposureApplyPhysicalCameraExposure` true :`AutoExposureLowPercent` 10.0 :`AutoExposureHighPercent` 90.0 :`AutoExposureMinBrightness` -10.0 :`AutoExposureMaxBrightness` 20.0 :`AutoExposureSpeedUp` 3.0 :`AutoExposureSpeedDown` 1.0 :`HistogramLogMin` -10.0 :`HistogramLogMax` 20.0 :`LocalExposureContrastScale` 1.0 :`LocalExposureDetailStrength` 1.0 :`LocalExposureBlurredLuminanceBlend` 0.6 :`LocalExposureBlurredLuminanceKernelSizePercent` 50.0 :`LensFlareIntensity` 1.0 :`LensFlareTint` (struct :`R` 1.0 :`G` 1.0 :`B` 1.0 :`A` 1.0) :`LensFlareBokehSize` 3.0 :`LensFlareThreshold` 8.0 :`LensFlareTints[0]` (struct :`R` 1.0 :`G` 0.8 :`B` 0.4 :`A` 0.6) :`LensFlareTints[1]` (struct :`R` 1.0 :`G` 1.0 :`B` 0.6 :`A` 0.53) :`LensFlareTints[2]` (struct :`R` 0.8 :`G` 0.8 :`B` 1.0 :`A` 0.46) :`LensFlareTints[3]` (struct :`R` 0.5 :`G` 1.0 :`B` 0.4 :`A` 0.39) :`LensFlareTints[4]` (struct :`R` 0.5 :`G` 0.8 :`B` 1.0 :`A` 0.31) :`LensFlareTints[5]` (struct :`R` 0.9 :`G` 1.0 :`B` 0.8 :`A` 0.27) :`LensFlareTints[6]` (struct :`R` 1.0 :`G` 0.8 :`B` 0.4 :`A` 0.22) :`LensFlareTints[7]` (struct :`R` 0.9 :`G` 0.7 :`B` 0.7 :`A` 0.15) :`VignetteIntensity` 0.4 :`FilmGrainIntensityShadows` 1.0 :`FilmGrainIntensityMidtones` 1.0 :`FilmGrainIntensityHighlights` 1.0 :`FilmGrainShadowsMax` 0.09 :`FilmGrainHighlightsMin` 0.5 :`FilmGrainHighlightsMax` 1.0 :`FilmGrainTexelSize` 1.0 :`AmbientOcclusionIntensity` 0.5 :`AmbientOcclusionStaticFraction` 1.0 :`AmbientOcclusionRadius` 200.0 :`AmbientOcclusionFadeDistance` 8000.0 :`AmbientOcclusionFadeRadius` 5000.0 :`AmbientOcclusionPower` 2.0 :`AmbientOcclusionBias` 3.0 :`AmbientOcclusionQuality` 50.0 :`AmbientOcclusionMipBlend` 0.6 :`AmbientOcclusionMipScale` 1.7 :`AmbientOcclusionMipThreshold` 0.01 :`AmbientOcclusionTemporalBlendWeight` 0.1 :`RayTracingAO` true :`RayTracingAOSamplesPerPixel` 1 :`RayTracingAOIntensity` 1.0 :`RayTracingAORadius` 200.0 :`ColorGradingIntensity` 1.0 :`DepthOfFieldSensorWidth` 24.576 :`DepthOfFieldDepthBlurAmount` 1.0 :`DepthOfFieldNearTransitionRegion` 300.0 :`DepthOfFieldFarTransitionRegion` 500.0 :`DepthOfFieldNearBlurSize` 15.0 :`DepthOfFieldFarBlurSize` 15.0 :`DepthOfFieldOcclusion` 0.4 :`DepthOfFieldVignetteSize` 200.0 :`MotionBlurAmount` 0.5 :`MotionBlurMax` 5.0 :`MotionBlurTargetFPS` 30 :`MotionBlurPerObjectSize` 0.5 :`TranslucencyType` "Raster" :`RayTracingTranslucencyMaxRoughness` 0.6 :`RayTracingTranslucencyRefractionRays` 3 :`RayTracingTranslucencySamplesPerPixel` 1 :`RayTracingTranslucencyShadows` "Hard_shadows" :`RayTracingTranslucencyRefraction` true :`PathTracingMaxBounces` 32 :`PathTracingSamplesPerPixel` 16384 :`PathTracingFilterWidth` 3.0 :`PathTracingEnableEmissive` true :`PathTracingMaxPathExposure` 30.0 :`PathTracingEnableDenoiser` true :`WeightedBlendables` (struct))))) _righteyedirection)))
          (bind (_returnvalue_x_3 _returnvalue_y_3 _returnvalue_z_3 _returnvalue_w_3) (`KismetMathLibrary.BreakVector4` (`KismetMathLibrary.Matrix_TransformVector` (`.ViewProjectionMatrix` (`GameplayStatics.GetViewProjectionMatrix` (make `MinimalViewInfo` _gazeorigin (struct) 110.0 512.0 0.0 2097152.0 1.0 true false "Perspective" 0.0 (struct :`BloomMethod` "BM_SOG" :`AutoExposureMethod` "AEM_Histogram" :`TemperatureType` "TEMP_WhiteBalance" :`WhiteTemp` 6500.0 :`ColorSaturation` (struct :`X` 1.0 :`Y` 1.0 :`Z` 1.0 :`W` 1.0) :`ColorContrast` (struct :`X` 1.0 :`Y` 1.0 :`Z` 1.0 :`W` 1.0) :`ColorGamma` (struct :`X` 1.0 :`Y` 1.0 :`Z` 1.0 :`W` 1.0) :`ColorGain` (struct :`X` 1.0 :`Y` 1.0 :`Z` 1.0 :`W` 1.0) :`ColorOffset` (struct) :`ColorSaturationShadows` (struct :`X` 1.0 :`Y` 1.0 :`Z` 1.0 :`W` 1.0) :`ColorContrastShadows` (struct :`X` 1.0 :`Y` 1.0 :`Z` 1.0 :`W` 1.0) :`ColorGammaShadows` (struct :`X` 1.0 :`Y` 1.0 :`Z` 1.0 :`W` 1.0) :`ColorGainShadows` (struct :`X` 1.0 :`Y` 1.0 :`Z` 1.0 :`W` 1.0) :`ColorOffsetShadows` (struct) :`ColorSaturationMidtones` (struct :`X` 1.0 :`Y` 1.0 :`Z` 1.0 :`W` 1.0) :`ColorContrastMidtones` (struct :`X` 1.0 :`Y` 1.0 :`Z` 1.0 :`W` 1.0) :`ColorGammaMidtones` (struct :`X` 1.0 :`Y` 1.0 :`Z` 1.0 :`W` 1.0) :`ColorGainMidtones` (struct :`X` 1.0 :`Y` 1.0 :`Z` 1.0 :`W` 1.0) :`ColorOffsetMidtones` (struct) :`ColorSaturationHighlights` (struct :`X` 1.0 :`Y` 1.0 :`Z` 1.0 :`W` 1.0) :`ColorContrastHighlights` (struct :`X` 1.0 :`Y` 1.0 :`Z` 1.0 :`W` 1.0) :`ColorGammaHighlights` (struct :`X` 1.0 :`Y` 1.0 :`Z` 1.0 :`W` 1.0) :`ColorGainHighlights` (struct :`X` 1.0 :`Y` 1.0 :`Z` 1.0 :`W` 1.0) :`ColorOffsetHighlights` (struct) :`ColorCorrectionHighlightsMin` 0.5 :`ColorCorrectionHighlightsMax` 1.0 :`ColorCorrectionShadowsMax` 0.09 :`BlueCorrection` 0.6 :`ExpandGamut` 1.0 :`ToneCurveAmount` 1.0 :`FilmSlope` 0.88 :`FilmToe` 0.55 :`FilmShoulder` 0.26 :`FilmWhiteClip` 0.04 :`SceneColorTint` (struct :`R` 1.0 :`G` 1.0 :`B` 1.0 :`A` 1.0) :`BloomIntensity` 0.675 :`BloomThreshold` -1.0 :`BloomSizeScale` 4.0 :`Bloom1Size` 0.3 :`Bloom2Size` 1.0 :`Bloom3Size` 2.0 :`Bloom4Size` 10.0 :`Bloom5Size` 30.0 :`Bloom6Size` 64.0 :`Bloom1Tint` (struct :`R` 0.3465 :`G` 0.3465 :`B` 0.3465 :`A` 1.0) :`Bloom2Tint` (struct :`R` 0.138 :`G` 0.138 :`B` 0.138 :`A` 1.0) :`Bloom3Tint` (struct :`R` 0.1176 :`G` 0.1176 :`B` 0.1176 :`A` 1.0) :`Bloom4Tint` (struct :`R` 0.066 :`G` 0.066 :`B` 0.066 :`A` 1.0) :`Bloom5Tint` (struct :`R` 0.066 :`G` 0.066 :`B` 0.066 :`A` 1.0) :`Bloom6Tint` (struct :`R` 0.061 :`G` 0.061 :`B` 0.061 :`A` 1.0) :`BloomConvolutionScatterDispersion` 1.0 :`BloomConvolutionSize` 1.0 :`BloomConvolutionCenterUV` (0.5 0.5) :`BloomConvolutionPreFilterMin` 7.0 :`BloomConvolutionPreFilterMax` 15000.0 :`BloomConvolutionPreFilterMult` 15.0 :`BloomConvolutionBufferScale` 0.133 :`BloomDirtMaskTint` (struct :`R` 0.5 :`G` 0.5 :`B` 0.5 :`A` 1.0) :`DynamicGlobalIlluminationMethod` "Lumen" :`IndirectLightingColor` (struct :`R` 1.0 :`G` 1.0 :`B` 1.0 :`A` 1.0) :`IndirectLightingIntensity` 1.0 :`LumenSceneLightingQuality` 1.0 :`LumenSceneDetail` 1.0 :`LumenSceneViewDistance` 20000.0 :`LumenSceneLightingUpdateSpeed` 1.0 :`LumenFinalGatherQuality` 1.0 :`LumenFinalGatherLightingUpdateSpeed` 1.0 :`LumenMaxTraceDistance` 20000.0 :`RayTracingGIType` "Disabled" :`RayTracingGIMaxBounces` 1 :`RayTracingGISamplesPerPixel` 4 :`ReflectionMethod` "Lumen" :`LumenReflectionQuality` 1.0 :`LumenRayLightingMode` "Default" :`ScreenSpaceReflectionIntensity` 100.0 :`ScreenSpaceReflectionQuality` 50.0 :`ScreenSpaceReflectionMaxRoughness` 0.6 :`RayTracingReflectionsMaxRoughness` 0.6 :`RayTracingReflectionsMaxBounces` 1 :`RayTracingReflectionsSamplesPerPixel` 1 :`RayTracingReflectionsShadows` "Hard_shadows" :`AmbientCubemapTint` (struct :`R` 1.0 :`G` 1.0 :`B` 1.0 :`A` 1.0) :`AmbientCubemapIntensity` 1.0 :`CameraShutterSpeed` 60.0 :`CameraISO` 100.0 :`DepthOfFieldFstop` 4.0 :`DepthOfFieldMinFstop` 1.2 :`DepthOfFieldBladeCount` 5 :`AutoExposureBias` 1.0 :`AutoExposureApplyPhysicalCameraExposure` true :`AutoExposureLowPercent` 10.0 :`AutoExposureHighPercent` 90.0 :`AutoExposureMinBrightness` -10.0 :`AutoExposureMaxBrightness` 20.0 :`AutoExposureSpeedUp` 3.0 :`AutoExposureSpeedDown` 1.0 :`HistogramLogMin` -10.0 :`HistogramLogMax` 20.0 :`LocalExposureContrastScale` 1.0 :`LocalExposureDetailStrength` 1.0 :`LocalExposureBlurredLuminanceBlend` 0.6 :`LocalExposureBlurredLuminanceKernelSizePercent` 50.0 :`LensFlareIntensity` 1.0 :`LensFlareTint` (struct :`R` 1.0 :`G` 1.0 :`B` 1.0 :`A` 1.0) :`LensFlareBokehSize` 3.0 :`LensFlareThreshold` 8.0 :`LensFlareTints[0]` (struct :`R` 1.0 :`G` 0.8 :`B` 0.4 :`A` 0.6) :`LensFlareTints[1]` (struct :`R` 1.0 :`G` 1.0 :`B` 0.6 :`A` 0.53) :`LensFlareTints[2]` (struct :`R` 0.8 :`G` 0.8 :`B` 1.0 :`A` 0.46) :`LensFlareTints[3]` (struct :`R` 0.5 :`G` 1.0 :`B` 0.4 :`A` 0.39) :`LensFlareTints[4]` (struct :`R` 0.5 :`G` 0.8 :`B` 1.0 :`A` 0.31) :`LensFlareTints[5]` (struct :`R` 0.9 :`G` 1.0 :`B` 0.8 :`A` 0.27) :`LensFlareTints[6]` (struct :`R` 1.0 :`G` 0.8 :`B` 0.4 :`A` 0.22) :`LensFlareTints[7]` (struct :`R` 0.9 :`G` 0.7 :`B` 0.7 :`A` 0.15) :`VignetteIntensity` 0.4 :`FilmGrainIntensityShadows` 1.0 :`FilmGrainIntensityMidtones` 1.0 :`FilmGrainIntensityHighlights` 1.0 :`FilmGrainShadowsMax` 0.09 :`FilmGrainHighlightsMin` 0.5 :`FilmGrainHighlightsMax` 1.0 :`FilmGrainTexelSize` 1.0 :`AmbientOcclusionIntensity` 0.5 :`AmbientOcclusionStaticFraction` 1.0 :`AmbientOcclusionRadius` 200.0 :`AmbientOcclusionFadeDistance` 8000.0 :`AmbientOcclusionFadeRadius` 5000.0 :`AmbientOcclusionPower` 2.0 :`AmbientOcclusionBias` 3.0 :`AmbientOcclusionQuality` 50.0 :`AmbientOcclusionMipBlend` 0.6 :`AmbientOcclusionMipScale` 1.7 :`AmbientOcclusionMipThreshold` 0.01 :`AmbientOcclusionTemporalBlendWeight` 0.1 :`RayTracingAO` true :`RayTracingAOSamplesPerPixel` 1 :`RayTracingAOIntensity` 1.0 :`RayTracingAORadius` 200.0 :`ColorGradingIntensity` 1.0 :`DepthOfFieldSensorWidth` 24.576 :`DepthOfFieldDepthBlurAmount` 1.0 :`DepthOfFieldNearTransitionRegion` 300.0 :`DepthOfFieldFarTransitionRegion` 500.0 :`DepthOfFieldNearBlurSize` 15.0 :`DepthOfFieldFarBlurSize` 15.0 :`DepthOfFieldOcclusion` 0.4 :`DepthOfFieldVignetteSize` 200.0 :`MotionBlurAmount` 0.5 :`MotionBlurMax` 5.0 :`MotionBlurTargetFPS` 30 :`MotionBlurPerObjectSize` 0.5 :`TranslucencyType` "Raster" :`RayTracingTranslucencyMaxRoughness` 0.6 :`RayTracingTranslucencyRefractionRays` 3 :`RayTracingTranslucencySamplesPerPixel` 1 :`RayTracingTranslucencyShadows` "Hard_shadows" :`RayTracingTranslucencyRefraction` true :`PathTracingMaxBounces` 32 :`PathTracingSamplesPerPixel` 16384 :`PathTracingFilterWidth` 3.0 :`PathTracingEnableEmissive` true :`PathTracingMaxPathExposure` 30.0 :`PathTracingEnableDenoiser` true :`WeightedBlendables` (struct))))) _gazedirection)))
          (`/Game/Blueprints/Gaze/BP_FixationTable.AddFixation` (`self.FixationTable`) (make `FixationData` _fixationpoint (`GameplayStatics.GetWorldDeltaSeconds`) (`GameplayStatics.GetTimeSeconds`) "null" (0.0 0.0 0.0) (struct) (0.0 0.0 0.0) (0.0 0.0 0.0) (0.0 0.0 0.0) (`KismetMathLibrary.GetDirectionUnitVector` _gazeorigin _fixationpoint) (`PlayerCameraManager.GetCameraLocation` _returnvalue) (`PlayerCameraManager.GetCameraRotation` _returnvalue) 0.0 0.0 (`KismetMathLibrary.MakeVector2D` (`KismetMathLibrary.SafeDivide` _returnvalue_x _returnvalue_w) (`KismetMathLibrary.SafeDivide` _returnvalue_y _returnvalue_w)) (`KismetMathLibrary.MakeVector2D` (`KismetMathLibrary.SafeDivide` _returnvalue_x_2 _returnvalue_w_2) (`KismetMathLibrary.SafeDivide` _returnvalue_y_2 _returnvalue_w_2)) (`KismetMathLibrary.MakeVector2D` (`KismetMathLibrary.SafeDivide` _returnvalue_x_3 _returnvalue_w_3) (`KismetMathLibrary.SafeDivide` _returnvalue_y_3 _returnvalue_w_3)))))))))

(fn `UserConstructionScript`)