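; BP_GazeChecker is an experiment target cube that registers when it has been looked at for long enough, with gaze detected as overlap on the cube.
; If lookable, overlap begin and end start and stop a dwell timer.
; Tick turns the cube black and flags it as looked once the dwell exceeds TimerValidation.
; The construction script creates the colored dynamic material, and OnReset restores color and clears both flags.
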(event `OnReset`
  (`MaterialInstanceDynamic.SetVectorParameterValue` (`self.Material`) "Color" (`self.Color`))
  (set `self.HasBeenLooked` false)
  (set `self.IsCurrentlyLooked` false))

(event `self.ReceiveTick`
  (params (DeltaSeconds :type "Float (single-precision)"))
  (if (`self.IsCurrentlyLooked`)
    (if (> (- (`GameplayStatics.GetTimeSeconds`) (`self.StartTimeLooked`)) (`self.TimerValidation`))
      (`MaterialInstanceDynamic.SetVectorParameterValue` :`self` (`self.Material`) :`ParameterName` "Color")
      (set `self.HasBeenLooked` true))))

(event `self.Cube.OnComponentBeginOverlap`
  (params (OverlappedComponent :type "PrimitiveComponent Object Reference") (OtherActor :type "Actor Object Reference") (OtherComp :type "PrimitiveComponent Object Reference") (OtherBodyIndex :type Integer) (bFromSweep :type Boolean) (SweepResult :type "HitResult Structure (by ref)"))
  (if (`self.IsLookable`)
    (set `self.StartTimeLooked` (`GameplayStatics.GetTimeSeconds`))
    (set `self.IsCurrentlyLooked` true)))

(event `self.Cube.OnComponentEndOverlap`
  (params (OverlappedComponent :type "PrimitiveComponent Object Reference") (OtherActor :type "Actor Object Reference") (OtherComp :type "PrimitiveComponent Object Reference") (OtherBodyIndex :type Integer))
  (if (`self.IsLookable`)
    (set `self.IsCurrentlyLooked` false)))

(fn `UserConstructionScript`
  (bind _returnvalue (`PrimitiveComponent.CreateDynamicMaterialInstance` (`self.Cube`) 0 "/Game/Materials/Colors/M_WhiteLight.M_WhiteLight" "None"))
  (bind _output_get (set `self.Material` _returnvalue))
  (`MaterialInstanceDynamic.SetVectorParameterValue` _output_get "Color" (`self.Color`)))