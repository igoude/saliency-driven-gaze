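; Experiment manager for a VR study that moves the participant between a Lobby and timed exploration levels.
; In Lobby, Space fades out and loads the next level through the game instance; elsewhere, Tick timers trigger the experiment event, then fade and return to Lobby.
; CameraFade and UpdateFade lerp a post-process material's Blend, and Enter resets checkers.
; Setup of that material, game instance and Lobby texts is disconnected from BeginPlay.
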(event `self.ReceiveBeginPlay`)

(event `Key|Enter`
  (params (Key :type "Key Structure"))
  (:`Pressed`
    (for _array_element (`self.Checkers`)
      (`/Game/Blueprints/Experiment/BP_GazeChecker.OnReset` _array_element))))

(event `Key|SpaceBar`
  (params (Key :type "Key Structure"))
  (bind _timerfading (`self.TimerFading`))
  (:`Pressed`
    (bind _returnvalue (`GameplayStatics.GetCurrentLevelName` true))
    (if (== _returnvalue "Lobby")
      (if (`KismetSystemLibrary.IsValid` (`self.GameInstance`))
        (`self.CameraFade` 0.0 1.0 _timerfading)
        (`KismetSystemLibrary.Delay` (+ _timerfading (`self.TimerLoading`)))
        (`/Game/Blueprints/GameMode/BP_ExperimentInstance.LoadNextLevel` (`self.GameInstance`))))))

(event `self.ReceiveTick`
  (params (DeltaSeconds :type "Float (single-precision)"))
  (bind _returnvalue (`self.GetGameTimeSinceCreation`))
  (bind _experimentevent (`self.ExperimentEvent`))
  (`|ExecutionSequence`
    (:`then_0`
      (`self.UpdateFade`))
    (:`then_1`
      (bind _returnvalue_2 (`GameplayStatics.GetCurrentLevelName` true))
      (if (!= _returnvalue_2 "Lobby")
        (`|ExecutionSequence`
          (:`then_0`
            (if (> _returnvalue (`self.TimerEvent`))
              (if (`KismetSystemLibrary.IsValid` _experimentevent)
                (if (not (`/Game/Blueprints/LevelEvents/BP_ExperimentEvent.IsTriggered` _experimentevent))
                  (`/Game/Blueprints/LevelEvents/BP_ExperimentEvent.OnEventTrigger` _experimentevent)))))
          (:`then_1`
            (if (> _returnvalue (`self.TimerExploration`))
              (if (`KismetSystemLibrary.IsValid` (`self.GameInstance`))
                (if (not (`self.WaitForLoby`))
                  (`self.CameraFade` 0.0 1.0 (`self.TimerFading`))
                  (set `self.WaitForLoby` true)
                  (set `self.TimerLobby` (`self.GetGameTimeSinceCreation`)))))))))))

(event `self.ReceiveEndPlay`
  (params (EndPlayReason :type "EEndPlayReason Enum" :default "Destroyed")))

(fn `CameraFade`
  (params (From :type "Float (double-precision)") (To :type "Float (double-precision)") (Time :type "Float (double-precision)"))
  (set `self.AlphaFrom` From)
  (set `self.AlphaCurrent` 0.0)
  (set `self.AlphaTo` To)
  (set `self.TimeStart` (`self.GetGameTimeSinceCreation`))
  (set `self.Timer` Time)
  (set `self.IsFading` true))

(fn `UpdateFade`
  (`|ExecutionSequence`
    (:`then_0`
      (if (`self.IsFading`)
        (bind _output_get (set `self.AlphaCurrent` (/ (- (`self.GetGameTimeSinceCreation`) (`self.TimeStart`)) (`self.Timer`))))
        (if (> _output_get 1.0)
          (set `self.IsFading` false)
          (`MaterialInstanceDynamic.SetScalarParameterValue` (`self.TransitionMaterial`) "Blend" (`self.AlphaTo`))
          (else
            (`MaterialInstanceDynamic.SetScalarParameterValue` (`self.TransitionMaterial`) "Blend" (`KismetMathLibrary.Lerp` (`self.AlphaFrom`) (`self.AlphaTo`) (`self.AlphaCurrent`)))))))
    (:`then_1`
      (if (`self.WaitForLoby`)
        (if (> (- (`self.GetGameTimeSinceCreation`) (`self.TimerLobby`)) (+ (`self.TimerLoading`) (`self.TimerFading`)))
          (`/Game/Blueprints/GameMode/BP_ExperimentInstance.LoadLobby` (`self.GameInstance`)))))))

(fn `UserConstructionScript`)