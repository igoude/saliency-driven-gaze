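; Game instance that sequences a participant's experiment through twelve level variants: three levels, each void or populated, with or without event.
; LoadNextLevel opens whichever level's ExperimentData order value matches LevelCounter, then increments it after a delay.
; LoadLobby returns to the lobby unless the counter is 12.
; FindExperimentRow takes the first not-Done data table row as the user and rewrites the table to CSV, but its only call here is unreachable.
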(event `self.ReceiveInit`)

(event `LoadNextLevel`
  (bind _levelcounter (`self.LevelCounter`))
  (bind (_experimentdata_done _experimentdata_level_1_void _experimentdata_level_1_populated _experimentdata_level_1_void_event _experimentdata_level_1_populated_event _experimentdata_level_2_void _experimentdata_level_2_populated _experimentdata_level_2_void_event _experimentdata_level_2_populated_event _experimentdata_level_3_void _experimentdata_level_3_populated _experimentdata_level_3_void_event _experimentdata_level_3_populated_event) (break `ExperimentData` (`self.ExperimentData`)))
  (if (== _levelcounter _experimentdata_level_1_void)
    (`GameplayStatics.OpenLevel` "Level_1_void")
    (`|ExecutionSequence` :!label _label
      (:`then_0`
        (`KismetSystemLibrary.Delay` 1.0)
        (`/Engine/EditorBlueprintResources/StandardMacros.IncrementInt` (`self.LevelCounter`))))
    (elif (== _levelcounter _experimentdata_level_1_populated)
      (`GameplayStatics.OpenLevel` "Level_1_populated")
      (goto _label)
      (elif (== _levelcounter _experimentdata_level_1_void_event)
        (`GameplayStatics.OpenLevel` "Level_1_void_event")
        (goto _label)
        (elif (== _levelcounter _experimentdata_level_1_populated_event)
          (`GameplayStatics.OpenLevel` "Level_1_populated_event")
          (goto _label)
          (elif (== _levelcounter _experimentdata_level_2_void)
            (`GameplayStatics.OpenLevel` "Level_2_void")
            (goto _label)
            (elif (== _levelcounter _experimentdata_level_2_populated)
              (`GameplayStatics.OpenLevel` "Level_2_populated")
              (goto _label)
              (elif (== _levelcounter _experimentdata_level_2_void_event)
                (`GameplayStatics.OpenLevel` "Level_2_void_event")
                (goto _label)
                (elif (== _levelcounter _experimentdata_level_2_populated_event)
                  (`GameplayStatics.OpenLevel` "Level_2_populated_event")
                  (goto _label)
                  (elif (== _levelcounter _experimentdata_level_3_void)
                    (`GameplayStatics.OpenLevel` "Level_3_void")
                    (goto _label)
                    (elif (== _levelcounter _experimentdata_level_3_populated)
                      (`GameplayStatics.OpenLevel` "Level_3_populated")
                      (goto _label)
                      (elif (== _levelcounter _experimentdata_level_3_void_event)
                        (`GameplayStatics.OpenLevel` "Level_3_void_event")
                        (goto _label)
                        (elif (== _levelcounter _experimentdata_level_3_populated_event)
                          (`GameplayStatics.OpenLevel` "Level_3_populated_event")
                          (goto _label))))))))))))))

(event `LoadLobby`
  (if (not (== (`self.LevelCounter`) 12))
    (`GameplayStatics.OpenLevel` "Lobby")))

(fn `FindExperimentRow`
  (locals (ExperimentRows :type "Array of  Structure") (UserIDs :type "Array of String") (UserFound :type Boolean))
  (bind _experimenttable (`self.ExperimentTable`))
  (bind _outrownames (`DataTableFunctionLibrary.GetDataTableRowNames` _experimenttable))
  (for _array_element _outrownames
    (bind _returnvalue (`|GetDataTableRow` _experimenttable _array_element)
      (:`then`
        (if (and (not (`local.UserFound`)) (== (`.Done` (break `ExperimentData` _returnvalue)) 0))
          (set `self.UserID` _array_element)
          (bind _output_get (set `self.ExperimentData` _returnvalue))
          (bind (_done _level_1_void _level_1_populated _level_1_void_event _level_1_populated_event _level_2_void _level_2_populated _level_2_void_event _level_2_populated_event _level_3_void _level_3_populated _level_3_void_event _level_3_populated_event) (break `ExperimentData` _output_get))
          (`KismetArrayLibrary.Array_Add` (`self.ExperimentArray`) (make `ExperimentData` 0 _level_1_void _level_1_populated _level_1_void_event _level_1_populated_event _level_2_void _level_2_populated _level_2_void_event _level_2_populated_event _level_3_void _level_3_populated _level_3_void_event _level_3_populated_event))
          (`KismetArrayLibrary.Array_Add` (`local.UserIDs`) (`KismetStringLibrary.Conv_NameToString` _array_element))
          (set `local.UserFound` true)
          (else
            (`KismetArrayLibrary.Array_Add` (`self.ExperimentArray`) _returnvalue)
            (`KismetArrayLibrary.Array_Add` (`local.UserIDs`) (`KismetStringLibrary.Conv_NameToString` _array_element)))))
      (:`RowNotFound`
        (`KismetSystemLibrary.PrintString` "UserID is undefined in the ExperimentTable"))))
  ;[1 1 1] !! Allow overwriting for the real experiment !!
  (`CsvFileHelper.SaveExperimentTableToCsvFile` (`KismetSystemLibrary.GetProjectDirectory`) (`KismetStringLibrary.Concat_StrStr` "Content/Tables/" "ExperimentTable.csv") (`local.UserIDs`) (`self.ExperimentArray`) true))