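; Game instance that drives batch simulation runs across a list of levels, opening the current level on Init.
; RestartLevel reloads the level for a set number of runs, then advances to the next, quitting after the last.
; Getters expose the current field of view, gamma, and saliency, gaze, inhibition and task weights from indexed arrays.
; An unconnected branch holds a sweep over weight combinations, so RestartLevel never changes those indices.
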(event `self.ReceiveInit`
  (`GameplayStatics.OpenLevel` (`KismetStringLibrary.Conv_StringToName` (`|GetArrayItem` (`self.LevelNames`) (`self.LevelCounter`)))))

(event `RestartLevel`
  (bind _output (`|GetArrayItem` (`self.LevelNames`) (`self.LevelCounter`)))
  (if (== (`self.SimuCounter`) (- (`self.NbSimu`) 1))
    (if (>= (`self.LevelCounter`) (- (`KismetArrayLibrary.Array_Length` (`self.LevelNames`)) 1))
      (`KismetSystemLibrary.QuitGame` null "Quit")
      (else
        (set `self.LevelCounter` (+ (`self.LevelCounter`) 1))
        (set `self.SimuCounter` 0)
        (`GameplayStatics.OpenLevel` (`KismetStringLibrary.Conv_StringToName` _output) :!label _label)
        (`KismetSystemLibrary.PrintString` (`KismetStringLibrary.Concat_StrStr` _output " | " (`KismetStringLibrary.Conv_DoubleToString` (`|GetArrayItem` (`self.WeightGaze_t`) (`self.WeightGazeCounter`))) " | " (`KismetStringLibrary.Conv_DoubleToString` (`|GetArrayItem` (`self.WeightSaliency_t`) (`self.WeightSaliencyCounter`))) " | " (`KismetStringLibrary.Conv_DoubleToString` (`|GetArrayItem` (`self.WeightInhibition_t`) (`self.WeightInhibitionCounter`))) " | " (`KismetStringLibrary.Conv_IntToString` (`self.SimuCounter`))))))
    (else
      (`/Engine/EditorBlueprintResources/StandardMacros.IncrementInt` (`self.SimuCounter`)
        (:`  `
          (goto _label))))))

(fn `GetCurrentFov`
  (returns (FoV :type "Float (double-precision)"))
  (return (`|GetArrayItem` (`self.FoV_t`) (`self.FoVCounter`))))

(fn `GetCurrentGamma`
  (returns (Gamma :type "Float (double-precision)"))
  (return (`|GetArrayItem` (`self.Gamma_t`) (`self.GammaCounter`))))

(fn `GetCurrentWeightGaze`
  (returns (GazeWeight :type "Float (double-precision)"))
  (return (`|GetArrayItem` (`self.WeightGaze_t`) (`self.WeightGazeCounter`))))

(fn `GetCurrentWeightInhibition`
  (returns (InhibitionWeight :type "Float (double-precision)"))
  (return (`|GetArrayItem` (`self.WeightInhibition_t`) (`self.WeightInhibitionCounter`))))

(fn `GetCurrentWeightSaliency`
  (returns (SaliencyWeight :type "Float (double-precision)"))
  (return (`|GetArrayItem` (`self.WeightSaliency_t`) (`self.WeightSaliencyCounter`))))

(fn `GetCurrentWeightTask`
  (returns (TaskWeight :type "Float (double-precision)"))
  (return (`|GetArrayItem` (`self.WeighTask_t`) (`self.WeightTaskCounter`))))