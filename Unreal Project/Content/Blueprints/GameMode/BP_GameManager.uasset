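; Manager for a MetaHuman gaze demo that drives the UI for switching levels, selecting a MetaHuman, tuning gaze map weights and quitting.
; BeginPlay creates the widget, gathers every actor's BP_MetaHumansGaze component and binds the controls.
; Weight sliders write to the selected gaze component and MyHUD, which shows debug maps when toggled.
; Selecting a MetaHuman eases the player pawn to face its nose socket over one second on Tick.
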(event `self.ReceiveBeginPlay`
  (bind _returnvalue (`GameplayStatics.GetPlayerController` 0))
  (bind _combometahumans (`/Game/Blueprints/GameMode/MyWidget.ComboMetaHumans` (`self.UIWidget`)))
  (bind _combolevel (`/Game/Blueprints/GameMode/MyWidget.ComboLevel` (`self.UIWidget`)))
  (`|ExecutionSequence`
    (:`then_0`
      ;[1 0.5 0] Init HUD
      (bind _asmy_hud (cast `/Game/Blueprints/GameMode/MyHUD` (`PlayerController.GetHUD` _returnvalue)))
      (set `self.MapsViewerHUD` _asmy_hud)
      (bind _returnvalue_2 (`|CreateWidget` "/Game/Blueprints/GameMode/MyWidget.MyWidget_C" _returnvalue))
      (bind _output_get (set `self.UIWidget` _returnvalue_2))
      (`UserWidget.AddToViewport` _output_get 0))
    (:`then_1`
      (bind _outactors (`GameplayStatics.GetAllActorsOfClass` "/Script/Engine.Actor"))
      (for _array_element _outactors
        (bind _returnvalue_3 (`self.GetComponentByClass` _array_element "/Game/Blueprints/Gaze/BP_MetaHumansGaze.BP_MetaHumansGaze_C"))
        (if (`KismetSystemLibrary.IsValid` _returnvalue_3)
          (`KismetArrayLibrary.Array_Add` (`self.MetaGazes`) _returnvalue_3)
          (`ComboBoxString.AddOption` _combometahumans (`KismetSystemLibrary.GetObjectName` _array_element))))
      (`ComboBoxString.SetSelectedOption` _combometahumans (`ComboBoxString.GetOptionAtIndex` _combometahumans 0)))
    (:`then_2`
      (bind _returnvalue_4 (`GameplayStatics.GetCurrentLevelName` true))
      (switch `string` _returnvalue_4
        (:`Lobby_demo`
          (`ComboBoxString.SetSelectedIndex` _combolevel 0))
        (:`Level_1_demo`
          (`ComboBoxString.SetSelectedIndex` _combolevel 1))
        (:`Level_2_demo`
          (`ComboBoxString.SetSelectedIndex` _combolevel 2))
        (:`Level_3_demo`
          (`ComboBoxString.SetSelectedIndex` _combolevel 3))))
    (:`then_3`
      ;[0 1 0.25] Change level
      (add `ComboBoxString.OnSelectionChanged` (`/Game/Blueprints/GameMode/MyWidget.ComboLevel` (`self.UIWidget`)) (delegate `OnLevelChanged`)))
    (:`then_4`
      ;[0 1 0.5] Change Debug mode
      (add `CheckBox.OnCheckStateChanged` (`/Game/Blueprints/GameMode/MyWidget.CheckBoxDebug` (`self.UIWidget`)) (delegate `OnDebugChanged`)))
    (:`then_5`
      ;[0 1 0.75] Change MetaHuman view
      (add `ComboBoxString.OnSelectionChanged` (`/Game/Blueprints/GameMode/MyWidget.ComboMetaHumans` (`self.UIWidget`)) (delegate `OnMetaHumanChanged`)))
    (:`then_6`
      ;[0 1 1] Change maps weights
      (add `Slider.OnValueChanged` (`/Game/Blueprints/GameMode/MyWidget.Slider_saliency` (`self.UIWidget`)) (delegate `OnSaliencyChanged`))
      (add `Slider.OnValueChanged` (`/Game/Blueprints/GameMode/MyWidget.Slider_saccadic` (`self.UIWidget`)) (delegate `OnSaccadicChanged`))
      (add `Slider.OnValueChanged` (`/Game/Blueprints/GameMode/MyWidget.Slider_inhibition` (`self.UIWidget`)) (delegate `OnInhibitionChanged`))
      (add `Slider.OnValueChanged` (`/Game/Blueprints/GameMode/MyWidget.Slider_bias` (`self.UIWidget`)) (delegate `OnBiasChanged`))
      (add `Slider.OnValueChanged` (`/Game/Blueprints/GameMode/MyWidget.Slider_desaturation` (`self.UIWidget`)) (delegate `OnDesaturationChanged`)))
    (:`then_7`
      ;[1 0 0] Quit game
      (add `Button.OnClicked` (`/Game/Blueprints/GameMode/MyWidget.QuitButton` (`self.UIWidget`)) (delegate `OnQuitClicked`)))
    (:`then_8`
      ;[0.5 0 1] Init HUD values
      (`self.UpdateMapsValues` (`|GetArrayItem` (`self.MetaGazes`) (`self.MetaGazeIndex`))))))

(event `OnLevelChanged`
  (params (SelectedItem :type String) (SelectionType :type "ESelectInfo Enum" :default "OnKeyPress"))
  ;[0 1 0.25] Change level
  (switch `string` SelectedItem
    (:`Lobby`
      (`GameplayStatics.OpenLevel` "Lobby_demo"))
    (:`Waiting room`
      (`GameplayStatics.OpenLevel` "Level_1_demo"))
    (:`Bar`
      (`GameplayStatics.OpenLevel` "Level_2_demo"))
    (:`Poker table`
      (`GameplayStatics.OpenLevel` "Level_3_demo"))))

(event `OnDebugChanged`
  (params (bIsChecked :type Boolean))
  (bind _mapsviewerhud (`self.MapsViewerHUD`))
  (bind _output (`|GetArrayItem` (`self.MetaGazes`) (`self.MetaGazeIndex`)))
  ;[0 1 0.5] Change Debug mode
  (if bIsChecked
    (set `/Game/Blueprints/GameMode/MyHUD.DrawDebugMaps` true _mapsviewerhud)
    (set `/Game/Blueprints/Gaze/BP_MetaHumansGaze.DrawSaliencyMap` true _output)
    (`/Game/Blueprints/Gaze/BP_MetaHumansGaze.DrawDebugMapsHUD` _output _mapsviewerhud)
    (`self.LookAtMetaHuman` _output)
    (else
      (set `/Game/Blueprints/GameMode/MyHUD.DrawDebugMaps` false _mapsviewerhud)
      (set `/Game/Blueprints/Gaze/BP_MetaHumansGaze.DrawSaliencyMap` false _output))))

(event `OnMetaHumanChanged`
  (params (SelectedItem :type String) (SelectionType :type "ESelectInfo Enum" :default "OnKeyPress"))
  (bind _metagazes (`self.MetaGazes`))
  (bind _output (`|GetArrayItem` _metagazes (`self.MetaGazeIndex`)))
  ;[0 1 0.75] Change MetaHuman view
  (set `self.MetaGazeIndex` (`ComboBoxString.GetSelectedIndex` (`/Game/Blueprints/GameMode/MyWidget.ComboMetaHumans` (`self.UIWidget`))))
  (`self.UpdateMapsValues` _output)
  (`self.LookAtMetaHuman` _output)
  (for _array_element _metagazes
    (set `/Game/Blueprints/Gaze/BP_MetaHumansGaze.DrawSaliencyMap` false _array_element))
  (`self.OnDebugChanged` (`CheckBox.IsChecked` (`/Game/Blueprints/GameMode/MyWidget.CheckBoxDebug` (`self.UIWidget`)))))

(event `OnSaliencyChanged`
  (params (Value :type "Float (single-precision)"))
  ;[0 1 1] Change maps weights
  (set `/Game/Blueprints/Gaze/BP_MetaHumansGaze.SaliencyWeight` Value (`|GetArrayItem` (`self.MetaGazes`) (`self.MetaGazeIndex`)))
  (set `/Game/Blueprints/GameMode/MyHUD.W_Saliency` Value (`self.MapsViewerHUD`)))

(event `OnSaccadicChanged`
  (params (Value :type "Float (single-precision)"))
  ;[0 1 1] Change maps weights
  (set `/Game/Blueprints/Gaze/BP_MetaHumansGaze.SaccadicWeight` Value (`|GetArrayItem` (`self.MetaGazes`) (`self.MetaGazeIndex`)))
  (set `/Game/Blueprints/GameMode/MyHUD.W_Saccadic` Value (`self.MapsViewerHUD`)))

(event `OnInhibitionChanged`
  (params (Value :type "Float (single-precision)"))
  ;[0 1 1] Change maps weights
  (set `/Game/Blueprints/Gaze/BP_MetaHumansGaze.InhibitionWeight` Value (`|GetArrayItem` (`self.MetaGazes`) (`self.MetaGazeIndex`)))
  (set `/Game/Blueprints/GameMode/MyHUD.W_Inhibition` Value (`self.MapsViewerHUD`)))

(event `OnBiasChanged`
  (params (Value :type "Float (single-precision)"))
  ;[0 1 1] Change maps weights
  (set `/Game/Blueprints/Gaze/BP_MetaHumansGaze.BiasWeight` Value (`|GetArrayItem` (`self.MetaGazes`) (`self.MetaGazeIndex`)))
  (set `/Game/Blueprints/GameMode/MyHUD.W_Biases` Value (`self.MapsViewerHUD`)))

(event `OnDesaturationChanged`
  (params (Value :type "Float (single-precision)"))
  ;[0 1 1] Change maps weights
  (set `/Game/Blueprints/GameMode/MyHUD.MapsDesaturation` Value (`self.MapsViewerHUD`)))

(event `OnQuitClicked`
  ;[1 0 0] Quit game
  (`KismetSystemLibrary.QuitGame` null "Quit"))

(event `self.ReceiveTick`
  (params (DeltaSeconds :type "Float (single-precision)"))
  (`self.UpdateCameraTransform`))

(fn `LookAtMetaHuman`
  (params (Metahuman :type "/Game/Blueprints/Gaze/BP_MetaHumansGaze Object Reference"))
  (bind _returnvalue (`GameplayStatics.GetPlayerController` 0))
  (bind _metahumanface (`/Game/Blueprints/Gaze/BP_MetaHumansGaze.MetaHumanFace` Metahuman))
  (bind _returnvalue_2 (`KismetMathLibrary.GetForwardVector` (`SceneComponent.GetSocketRotation` _metahumanface "Face_Nose_Socket")))
  (`|ExecutionSequence`
    (:`then_0`
      (set `self.CameraTimer` 0.0))
    (:`then_1`
      (set `self.InitCameraLocation` (`self.K2_GetActorLocation` (`Controller.K2_GetPawn` _returnvalue)))
      (set `self.InitCameraRotation` (`Controller.GetControlRotation` _returnvalue)))
    (:`then_2`
      (set `self.FinalCameraLocation` (+ (`SceneComponent.GetSocketLocation` _metahumanface "Face_Nose_Socket") (* _returnvalue_2 50.0)))
      (set `self.FinalCameraRotation` (`KismetMathLibrary.Conv_VectorToRotator` (`KismetMathLibrary.NegateVector` _returnvalue_2))))))

(fn `UpdateCameraTransform`
  (bind _returnvalue (`GameplayStatics.GetPlayerController` 0))
  (if (< (`self.CameraTimer`) 1.0)
    (`|ExecutionSequence`
      (:`then_0`
        (set `self.CameraTimer` (+ (`self.CameraTimer`) (`GameplayStatics.GetWorldDeltaSeconds`))))
      (:`then_1`
        (`self.K2_SetActorLocation` (`Controller.K2_GetPawn` _returnvalue) (`|EaseFunction` "EaseInOut" (`self.CameraTimer`) (`self.InitCameraLocation`) (`self.FinalCameraLocation`)) false false))
      (:`then_2`
        (`Controller.SetControlRotation` _returnvalue (`|EaseFunction` "EaseInOut" (`self.CameraTimer`) (`self.InitCameraRotation`) (`self.FinalCameraRotation`)))))))

(fn `UpdateMapsValues`
  (params (Metahuman :type "/Game/Blueprints/Gaze/BP_MetaHumansGaze Object Reference"))
  (bind _uiwidget (`self.UIWidget`))
  (`Slider.SetValue` (`/Game/Blueprints/GameMode/MyWidget.Slider_saliency` _uiwidget) (`/Game/Blueprints/Gaze/BP_MetaHumansGaze.SaliencyWeight` Metahuman))
  (`Slider.SetValue` (`/Game/Blueprints/GameMode/MyWidget.Slider_saccadic` _uiwidget) (`/Game/Blueprints/Gaze/BP_MetaHumansGaze.SaccadicWeight` Metahuman))
  (`Slider.SetValue` (`/Game/Blueprints/GameMode/MyWidget.Slider_inhibition` _uiwidget) (`/Game/Blueprints/Gaze/BP_MetaHumansGaze.InhibitionWeight` Metahuman))
  (`Slider.SetValue` (`/Game/Blueprints/GameMode/MyWidget.Slider_bias` _uiwidget) (`/Game/Blueprints/Gaze/BP_MetaHumansGaze.BiasWeight` Metahuman)))

(fn `UserConstructionScript`)