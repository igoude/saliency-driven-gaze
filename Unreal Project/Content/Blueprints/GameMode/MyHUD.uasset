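; Debug HUD that displays visual attention maps (saliency, saccadic, inhibition, biases and F_map) as labeled square panels along the screen's left and right edges.
; BeginPlay creates a dynamic material instance per panel, with saliency, inhibition and biases sharing the M_SaliencyOverlay parent.
; When DrawDebugMaps is set, DrawHUD sizes panels from screen height and calls per-map functions that push weights, desaturation and textures into each material before drawing it.
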(event `self.ReceiveBeginPlay`
  (`|ExecutionSequence`
    (:`then_0`
      (bind _returnvalue (`KismetMaterialLibrary.CreateDynamicMaterialInstance` "/Game/Materials/HUD/M_SaliencyOverlay.M_SaliencyOverlay"))
      (set `self.SaliencyMaterial` _returnvalue))
    (:`then_1`
      (bind _returnvalue_2 (`KismetMaterialLibrary.CreateDynamicMaterialInstance` "/Game/Materials/HUD/M_SaccadicOverlay.M_SaccadicOverlay"))
      (set `self.SaccadicMaterial` _returnvalue_2))
    (:`then_2`
      (bind _returnvalue_3 (`KismetMaterialLibrary.CreateDynamicMaterialInstance` "/Game/Materials/HUD/M_SaliencyOverlay.M_SaliencyOverlay"))
      (set `self.InhibitionMaterial` _returnvalue_3))
    (:`then_3`
      (bind _returnvalue_4 (`KismetMaterialLibrary.CreateDynamicMaterialInstance` "/Game/Materials/HUD/M_SaliencyOverlay.M_SaliencyOverlay"))
      (set `self.BiasesMaterial` _returnvalue_4))
    (:`then_4`
      (bind _returnvalue_5 (`KismetMaterialLibrary.CreateDynamicMaterialInstance` "/Game/Materials/HUD/M_DistributionOverlay.M_DistributionOverlay"))
      (set `self.FmapMaterial` _returnvalue_5))))

(event `self.ReceiveDrawHUD`
  (params (SizeX :type Integer) (SizeY :type Integer))
  (bind _returnvalue (/ (`KismetMathLibrary.Conv_IntToDouble` SizeY) 3.0))
  (bind _returnvalue_2 (- _returnvalue 10.0))
  (bind _returnvalue_3 (- (`KismetMathLibrary.Conv_IntToDouble` SizeX) (+ _returnvalue_2 5.0)))
  (if (`self.DrawDebugMaps`)
    (`|ExecutionSequence`
      (:`then_0`
        (`self.DrawSaliency` 5.0 5.0 _returnvalue_2 _returnvalue_2))
      (:`then_1`
        (`self.DrawSaccadic` 5.0 _returnvalue _returnvalue_2 _returnvalue_2))
      (:`then_2`
        (`self.DrawInhibition` 5.0 (+ _returnvalue _returnvalue) _returnvalue_2 _returnvalue_2))
      (:`then_3`
        (`self.DrawBiases` _returnvalue_3 5.0 _returnvalue_2 _returnvalue_2))
      (:`then_4`
        (`self.DrawFMap` _returnvalue_3 _returnvalue _returnvalue_2 _returnvalue_2)))))

(fn `DrawBiases`
  (params (ScreenX :type "Float (double-precision)") (ScreenY :type "Float (double-precision)") (ScreenW :type "Float (double-precision)") (ScreenH :type "Float (double-precision)"))
  (bind _biasesmaterial (`self.BiasesMaterial`))
  (`MaterialInstanceDynamic.SetScalarParameterValue` _biasesmaterial "Weight" (`self.W_Biases`))
  (`MaterialInstanceDynamic.SetScalarParameterValue` _biasesmaterial "Desaturation" (`self.MapsDesaturation`))
  (`MaterialInstanceDynamic.SetTextureParameterValue` _biasesmaterial "View" (`self.View`))
  (`MaterialInstanceDynamic.SetTextureParameterValue` _biasesmaterial "Saliency" (`self.Biases`))
  (`self.DrawMaterial` _biasesmaterial ScreenX ScreenY ScreenW ScreenH 0.0 0.0 1.0 1.0)
  (`self.DrawText` "Biases" (struct :`R` 1.0 :`G` 1.0 :`B` 1.0 :`A` 1.0) (+ ScreenX 5.0) (+ ScreenY 5.0) null))

(fn `DrawFMap`
  (params (ScreenX :type "Float (double-precision)") (ScreenY :type "Float (double-precision)") (ScreenW :type "Float (double-precision)") (ScreenH :type "Float (double-precision)"))
  (bind _fmapmaterial (`self.FmapMaterial`))
  (`MaterialInstanceDynamic.SetScalarParameterValue` _fmapmaterial "SaliencyWeight" (`self.W_Saliency`))
  (`MaterialInstanceDynamic.SetScalarParameterValue` _fmapmaterial "Desaturation" (`self.MapsDesaturation`))
  (`MaterialInstanceDynamic.SetTextureParameterValue` _fmapmaterial "View" (`self.View`))
  (`MaterialInstanceDynamic.SetTextureParameterValue` _fmapmaterial "Saliency" (`self.Saliency`))
  (`MaterialInstanceDynamic.SetTextureParameterValue` _fmapmaterial "Distribution" (`self.Blend`))
  (`self.DrawMaterial` _fmapmaterial ScreenX ScreenY ScreenW ScreenH 0.0 0.0 1.0 1.0)
  (`self.DrawText` "F_map" (struct :`R` 1.0 :`G` 1.0 :`B` 1.0 :`A` 1.0) (+ ScreenX 5.0) (+ ScreenY 5.0) null))

(fn `DrawInhibition`
  (params (ScreenX :type "Float (double-precision)") (ScreenY :type "Float (double-precision)") (ScreenW :type "Float (double-precision)") (ScreenH :type "Float (double-precision)"))
  (bind _inhibitionmaterial (`self.InhibitionMaterial`))
  (`MaterialInstanceDynamic.SetScalarParameterValue` _inhibitionmaterial "Weight" (`self.W_Inhibition`))
  (`MaterialInstanceDynamic.SetScalarParameterValue` _inhibitionmaterial "Desaturation" (`self.MapsDesaturation`))
  (`MaterialInstanceDynamic.SetTextureParameterValue` _inhibitionmaterial "View" (`self.View`))
  (`MaterialInstanceDynamic.SetTextureParameterValue` _inhibitionmaterial "Saliency" (`self.Inhibition`))
  (`self.DrawMaterial` _inhibitionmaterial ScreenX ScreenY ScreenW ScreenH 0.0 0.0 1.0 1.0)
  (`self.DrawText` "Inhibition" (struct :`R` 1.0 :`G` 1.0 :`B` 1.0 :`A` 1.0) (+ ScreenX 5.0) (+ ScreenY 5.0) null))

(fn `DrawSaccadic`
  (params (ScreenX :type "Float (double-precision)") (ScreenY :type "Float (double-precision)") (ScreenW :type "Float (double-precision)") (ScreenH :type "Float (double-precision)"))
  (bind _saccadicmaterial (`self.SaccadicMaterial`))
  (`MaterialInstanceDynamic.SetScalarParameterValue` _saccadicmaterial "Weight" (`self.W_Saccadic`))
  (`MaterialInstanceDynamic.SetScalarParameterValue` _saccadicmaterial "Desaturation" (`self.MapsDesaturation`))
  (`MaterialInstanceDynamic.SetTextureParameterValue` _saccadicmaterial "View" (`self.View`))
  (`self.DrawMaterial` _saccadicmaterial ScreenX ScreenY ScreenW ScreenH 0.0 0.0 1.0 1.0)
  (`self.DrawText` "Saccadic" (struct :`R` 1.0 :`G` 1.0 :`B` 1.0 :`A` 1.0) (+ ScreenX 5.0) (+ ScreenY 5.0) null))

(fn `DrawSaliency`
  (params (ScreenX :type "Float (double-precision)") (ScreenY :type "Float (double-precision)") (ScreenW :type "Float (double-precision)") (ScreenH :type "Float (double-precision)"))
  (bind _saliencymaterial (`self.SaliencyMaterial`))
  (`MaterialInstanceDynamic.SetScalarParameterValue` _saliencymaterial "Weight" (`self.W_Saliency`))
  (`MaterialInstanceDynamic.SetScalarParameterValue` _saliencymaterial "Desaturation" (`self.MapsDesaturation`))
  (`MaterialInstanceDynamic.SetTextureParameterValue` _saliencymaterial "View" (`self.View`))
  (`MaterialInstanceDynamic.SetTextureParameterValue` _saliencymaterial "Saliency" (`self.Saliency`))
  (`self.DrawMaterial` _saliencymaterial ScreenX ScreenY ScreenW ScreenH 0.0 0.0 1.0 1.0)
  (`self.DrawText` "Saliency" (struct :`R` 1.0 :`G` 1.0 :`B` 1.0 :`A` 1.0) (+ ScreenX 5.0) (+ ScreenY 5.0) null))

(fn `UserConstructionScript`)